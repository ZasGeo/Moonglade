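; Grabbable boat control ring that a VR motion controller picks up and that returns to its left or right rope when dropped.
; Pickup and Drop fire dispatchers, set InHand and share one attach path, where a timeline lerps the ring's location and rotation to the new parent.
; Flicker drives U_Speed on the ring and sphere dynamic materials, StopFlicker swaps both to metal, and Restart restores the ring material.
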(event Custom|Flicker
  (Rendering|Material|SetScalarParameterValue (Variables|Default|GetM_Ring) "U_Speed" 0.35 :!class /Script/Engine.MaterialInstanceDynamic))

(event Custom|Restart
  (bind _sphere (Variables|Default|GetSphere))
  (bind _ring (Variables|Default|GetRing))
  (Variables|Default|SetInHand false)
  (Rendering|Material|SetMaterial (Variables|Default|GetRing) 0 "/Game/Geometry/Boat/M_Ring.M_Ring")
  (bind _returnvalue (Rendering|Material|CreateDynamicMaterialInstance _ring 0 (Rendering|Material|GetMaterial _ring 0) :!class /Script/Engine.PrimitiveComponent))
  (Variables|Default|SetM_Ring _returnvalue)
  (bind _returnvalue_2 (Rendering|Material|CreateDynamicMaterialInstance _sphere 0 (Rendering|Material|GetMaterial _sphere 0) :!class /Script/Engine.PrimitiveComponent))
  (Variables|Default|SetM_Sphere _returnvalue_2))

(event Custom|StopFlicker
  (Rendering|Material|SetMaterial (Variables|Default|GetRing) 0 "/Game/Geometry/Enviroment/M_Metail.M_Metail"))

(event EventPickup
  (params (AttachTo :type Scene%20Component%20Object%20Reference))
  (Variables|Default|SetAttachedTo AttachTo)
  (Default|CallPick)
  (Variables|Default|SetInHand true)
  (Transformation|AttachComponentToComponent (Variables|Default|GetAttachedTo) "None" "KeepWorld" "KeepWorld" "KeepWorld" false)
  (bind _newtrack_0 (Timeline|AttachTime PlayFromStart)
    (:Update
      (Transformation|SetActorLocation (Math|Vector|Lerp(Vector) (Transformation|GetActorLocation) (Transformation|GetWorldLocation (Variables|Default|GetAttachedTo)) _newtrack_0) false true)
      (Transformation|SetActorRotation (Math|Rotator|Lerp(Rotator) (Transformation|GetActorRotation) (Transformation|GetWorldRotation (Variables|Default|GetAttachedTo)) _newtrack_0 true) true))))

(event EventDrop
  (bind _controller (Variables|Default|GetController))
  (Variables|Default|SetAttachedTo (Utilities|Select :Index (Variables|Default|GetLeft/Right) :Left (Variables|/Game/Blueprints/Boat/BP_Pawn_VRBoat.BP_Pawn_VRBoat_C|GetLeftRope _controller) :Right (Variables|/Game/Blueprints/Boat/BP_Pawn_VRBoat.BP_Pawn_VRBoat_C|GetRightRope _controller) :Pad 0 :ExternalCamera 0 :Gun 0 :Special_1 0 :Special_2 0 :Special_3 0 :Special_4 0 :Special_5 0 :Special_6 0 :Special_7 0 :Special_8 0 :Special_9 0))
  (Default|CallDropD)
  (Variables|Default|SetInHand false)
  (Transformation|AttachComponentToComponent (Variables|Default|GetAttachedTo) "None" "KeepWorld" "KeepWorld" "KeepWorld" false)
  (bind _newtrack_0 (Timeline|AttachTime PlayFromStart)
    (:Update
      (Transformation|SetActorLocation (Math|Vector|Lerp(Vector) (Transformation|GetActorLocation) (Transformation|GetWorldLocation (Variables|Default|GetAttachedTo)) _newtrack_0) false true)
      (Transformation|SetActorRotation (Math|Rotator|Lerp(Rotator) (Transformation|GetActorRotation) (Transformation|GetWorldRotation (Variables|Default|GetAttachedTo)) _newtrack_0 true) true))))

(fn ConstructionScript
  (bind _sphere (Variables|Default|GetSphere))
  (bind _ring (Variables|Default|GetRing))
  (bind _returnvalue (Rendering|Material|CreateDynamicMaterialInstance _ring 0 (Rendering|Material|GetMaterial _ring 0) :!class /Script/Engine.PrimitiveComponent))
  (Variables|Default|SetM_Ring _returnvalue)
  (bind _returnvalue_2 (Rendering|Material|CreateDynamicMaterialInstance _sphere 0 (Rendering|Material|GetMaterial _sphere 0) :!class /Script/Engine.PrimitiveComponent))
  (Variables|Default|SetM_Sphere _returnvalue_2))