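; BP_Pawn_NVRBoat1 is a boat pawn that starts sailing and adjusts its two ropes from keyboard or gamepad input.
; H or the gamepad bottom face button triggers a one-time StartSail and SetGameMode, then raises both rope-end actors.
; The KeyBoard axis slides the left and right rope components in opposite directions along local Y within clamped limits.
; BeginPlay, Tick and overlap events are disabled, and a rope-end offset branch is unconnected.
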(event EventBeginPlay
  (|CallParentFunction))

(event Collision|EventActorBeginOverlap
  (params (OtherActor :type Actor%20Object%20Reference)))

(event EventTick
  (params (DeltaSeconds :type Float%20%28single-precision%29))
  (|CallParentFunction DeltaSeconds))

(event Input|AxisEvents|InputAxisKeyBoard
  (params (AxisValue :type Float%20%28single-precision%29))
  (bind _returnvalue (* AxisValue 2.0))
  (bind _leftrope (Variables|Default|GetLeftRope))
  (bind _rightrope (Variables|Default|GetRightRope))
  (bind _relativelocation (Variables|/Script/Engine.SceneComponent|GetRelativeLocation _rightrope))
  (bind _relativelocation_2 (Variables|/Script/Engine.SceneComponent|GetRelativeLocation _leftrope))
  (Transformation|SetRelativeLocation _leftrope (Math|Vector|MakeVector (.x _relativelocation_2) (Math|Float|Clamp(Float) (+ (.y _relativelocation_2) (* _returnvalue -1.0)) -1e+02 1e+02) (.z _relativelocation_2)) false false)
  (Transformation|SetRelativeLocation (Variables|Default|GetRightRope) (Math|Vector|MakeVector (.x _relativelocation) (Math|Float|Clamp(Float) (+ _returnvalue (.y _relativelocation)) -1e+02 1e+02) (.z _relativelocation)) false false))

(event Input|KeyboardEvents|H
  (params (Key :type Key%20Structure :default "AnyKey"))
  (:Pressed
    (Utilities|FlowControl|DoOnce false
      (:Completed
        (CallFunction|StartSail)
        (CallFunction|SetGameMode)
        (Transformation|AddActorWorldOffset (Variables|Default|GetRopeEndLeft) "0,0.000000,50.000000")))))

(event Input|GamepadEvents|GamepadFaceButtonBottom
  (params (Key :type Key%20Structure :default "AnyKey"))
  (:Pressed
    (Utilities|FlowControl|DoOnce false
      (:Completed
        (CallFunction|StartSail)
        (CallFunction|SetGameMode)
        (Transformation|AddActorWorldOffset (Variables|Default|GetRopeEndLeft) "0,0.000000,50.000000")))))

(fn ConstructionScript
  (|CallParentFunction))