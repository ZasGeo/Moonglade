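; BP_Ray is a boat component actor: a timed laser weapon that auto-fires at actors carrying BP_AC_OnRay.
; Activate enables collision for a set duration; Deactivate clears targets and charge.
; Sphere overlaps maintain the target list and start a timer-driven charge-and-fire loop, which holds its charge when no target qualifies.
; Each shot picks the nearest target inside a forward cone, calls its OnFire and aims the beam emitter at the returned actor.
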(event OnComponentBeginOverlap(Sphere)
  (params (OverlappedComponent :type Primitive%20Component%20Object%20Reference) (OtherActor :type Actor%20Object%20Reference) (OtherComp :type Primitive%20Component%20Object%20Reference) (OtherBodyIndex :type Integer) (bFromSweep :type Boolean) (SweepResult :type Hit%20Result%20Structure%20%28by%20ref%29))
  (bind _returnvalue (Actor|GetComponentbyClass OtherActor "/Game/Blueprints/levelGenerator/ObstacleItems/Components/BP_AC_OnRay.BP_AC_OnRay_C"))
  (Utilities|IsValid _returnvalue
    (:Is%20Valid
      (Utility|AddtoTargets _returnvalue)
      (CallFunction|StartFire))))

(event OnComponentEndOverlap(Sphere)
  (params (OverlappedComponent :type Primitive%20Component%20Object%20Reference) (OtherActor :type Actor%20Object%20Reference) (OtherComp :type Primitive%20Component%20Object%20Reference) (OtherBodyIndex :type Integer))
  (bind _returnvalue (Actor|GetComponentbyClass OtherActor "/Game/Blueprints/levelGenerator/ObstacleItems/Components/BP_AC_OnRay.BP_AC_OnRay_C"))
  (Utilities|IsValid _returnvalue
    (:Is%20Valid
      (Utility|RemovefromTargets _returnvalue))))

(event EventActivate
  (Collision|SetActorEnableCollision true)
  (CallFunction|StartFire)
  (Utilities|Time|ClearandInvalidateTimerbyHandle (Variables|Default|GetTimer))
  (bind _returnvalue (Utilities|Time|SetTimerbyFunctionName 0 "Deactivate" (Variables|Settings|GetDuration)))
  (Variables|Default|SetTimer _returnvalue))

(event EventDeactivate
  (Collision|SetActorEnableCollision false)
  (Utilities|Time|ClearandInvalidateTimerbyHandle (Variables|Default|GetChargeTimer))
  (Variables|Default|SetCharged false)
  (Utilities|Array|Clear (Variables|Default|GetTargets))
  (Components|Activation|SetActive (Variables|Default|GetP_Beam_Laser_Fire_Large) false false))

(event EventBeginPlay)

(fn ConstructionScript
  (Variables|Default|SetCosine (Math|Trig|Cos(Degrees) (/ (Variables|Settings|GetAngle) 2.0)))
  (Components|Sphere|SetSphereRadius (Variables|Default|GetSphere) (Variables|Settings|GetRadius) false)
  (CallFunction|Deactivate)
  (Effects|Components|ParticleSystem|SetFloatParameter (Variables|Default|GetP_Beam_Laser_Fire_Large) "Lifetime" (Variables|Settings|GetChargeTime)))

(fn GetTarget
  (for _array_element (Variables|Default|GetTargets)
    (if (>= (Math|Vector|DotProduct (Math|Vector|Normalize (- (Default|GetPos _array_element) (Transformation|GetActorLocation))) (Math|Vector|GetForwardVector (Variables|Default|GetArrow))) (Variables|Default|GetCosine))
      (Utilities|Array|Add (LocalVariables|GetInSector) _array_element)))
  (for _array_element_2 (LocalVariables|GetInSector)
    (if (<= (Math|Vector|VectorLengthSquared (- (Default|GetPos _array_element_2) (Transformation|GetActorLocation))) (LocalVariables|GetNearestDist))
      (LocalVariables|SetNearest _array_element_2)
      (LocalVariables|SetNearestDist (Math|Vector|VectorLengthSquared (- (Default|GetPos _array_element_2) (Transformation|GetActorLocation))))))
  (return (LocalVariables|GetNearest)))

(fn Charge
  (Development|PrintString "Charge")
  (bind _returnvalue (Utilities|Time|SetTimerbyFunctionName 0 "OnCharged" (Variables|Settings|GetChargeTime)))
  (Variables|Default|SetChargeTimer _returnvalue)
  (Components|Activation|SetActive (Variables|Default|GetP_Beam_Laser_Fire_Large) true true))

(fn Fire
  (bind _target (Utility|GetTarget))
  (Utilities|IsValid _target
    (:Is%20Valid
      (Development|PrintString "Fire")
      (bind _returnvalue (Default|OnFire _target))
      (Variables|Default|SetCharged false)
      (bind _returnvalue_2 (Effects|SpawnEmitteratLocation "/Game/InfinityBladeEffects/Effects/FX_Monsters/FX_Monster_Elemental/Fire/P_Beam_Laser.P_Beam_Laser" (Transformation|GetWorldLocation (Variables|Default|GetDefaultSceneRoot))))
      (Effects|Components|ParticleSystem|SetActorParameter _returnvalue_2 "Target" _returnvalue)
      (CallFunction|Charge))
    (:Is%20Not%20Valid
      (CallFunction|StopFire))))

(fn RemovefromTargets
  (params (Target :type BP%20AC%20on%20Ray%20Object%20Reference))
  (Utilities|Array|RemoveItem (Variables|Default|GetTargets) Target))

(fn AddtoTargets
  (params (Target :type BP%20AC%20on%20Ray%20Object%20Reference))
  (Utilities|Array|Add (Variables|Default|GetTargets) Target))

(fn OnCharged
  (Variables|Default|SetCharged true)
  (CallFunction|Fire))

(fn StartFire
  (Development|PrintString "StartFire")
  (if (not (Class|KismetSystemLibrary|TimerExistsHandle (Variables|Default|GetChargeTimer)))
    (if (Variables|Default|GetCharged)
      (CallFunction|Fire)
      (else
        (CallFunction|Charge)))))

(fn StopFire
  (Development|PrintString "StopFire"))