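; Boat health component that tracks separate damage for the left and right sides.
; Init stores the boat and its health material instance, then fills both sides to their maximums.
; Collision decrements the struck side and returns whether its health has dropped below zero.
; Each hit also raises that side's material mask parameter and spawns a random crack through the boat's BP_CrackDecal child actor.
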(fn Init
  (params (M_Health :type Material%20Instance%20Dynamic%20Object%20Reference) (Boat :type BP%20Pawn%20VR%20Boat%20Object%20Reference))
  (Variables|Default|SetM_Health M_Health)
  (Variables|Default|SetBoat Boat)
  (Variables|Default|SetLeftHealth (Variables|Default|GetMaxLeftHealth))
  (Variables|Default|SetRightHealth (Variables|Default|GetMaxRightHealth)))

(fn Collision
  (params (IsLeft :type Boolean))
  (CallFunction|SetMaterial IsLeft)
  (if IsLeft
    (bind _result (Math|Integer|DecrementInt (Variables|Default|GetLeftHealth))
      (:%20%20
        (LocalVariables|SetHealth _result)))
    (else
      (bind _result_2 (Math|Integer|DecrementInt (Variables|Default|GetRightHealth))
        (:%20%20
          (LocalVariables|SetHealth _result_2)))))
  (return (< (LocalVariables|GetHealth) 0)))

(fn SetMaterial
  (params (Isleft :type Boolean))
  (bind _output_get (LocalVariables|SetL_ParamName (select Isleft "MaskLeft" "MaskRight")))
  (bind _returnvalue (Rendering|Material|GetScalarParameterValue (Variables|Default|GetM_Health) _output_get :!class /Script/Engine.MaterialInstanceDynamic))
  (Rendering|Material|SetScalarParameterValue (Variables|Default|GetM_Health) (LocalVariables|GetL_ParamName) (+ _returnvalue 0.25) :!class /Script/Engine.MaterialInstanceDynamic)
  (bind _asbp_crack_decal (Utilities|Casting|CastToBP_CrackDecal (Variables|/Script/Engine.ChildActorComponent|GetChildActor (Variables|/Game/Blueprints/Boat/BP_Pawn_VRBoat.BP_Pawn_VRBoat_C|GetCracks (Variables|Default|GetBoat)))))
  (if Isleft
    (Default|RandomCrackLeft _asbp_crack_decal)
    (else
      (Default|RandomCrackRight _asbp_crack_decal))))