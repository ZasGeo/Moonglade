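; BP_Shield is a boat shield component that tracks a pool of charges for blocking.
; Add and remove functions keep the charge count clamped between zero and the maximum.
; A shield check spends one charge when available, exposed both as a boolean function (Shield1) and as a macro-style Shield graph that branches to Block or No.
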(fn AddShieldCharges
  (params (Charges :type Integer))
  (Variables|Default|SetShieldCharges (Math|Integer|Clamp(Integer) (+ (Variables|Default|GetShieldCharges) Charges) 0 (Variables|Default|GetShieldMaxCharges))))

(fn RemoveShieldCharges
  (params (Charges :type Integer))
  (Variables|Default|SetShieldCharges (Math|Integer|Clamp(Integer) (- (Variables|Default|GetShieldCharges) Charges) 0 (Variables|Default|GetShieldMaxCharges))))

(fn HasCharges
  (params (Charges :type Integer))
  (return (>= (Variables|Default|GetShieldCharges) Charges)))

(fn Shield1
  (bind _returnvalue (CallFunction|HasCharges 1))
  (if _returnvalue
    (CallFunction|RemoveShieldCharges 1)
    (return true)
    (else
      (return false))))