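; BP_Magneet is a boat magnet that pulls in eligible actors through a sphere trigger.
; Actors entering the sphere that carry a BP_AC_OnMagneet component have Start called on it with the boat and an acceleration, leaving the movement to that component.
; Activate widens the radius and restarts a duration timer that calls Deactivate to shrink it back.
; Construction starts it in the deactivated state.
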(event OnComponentBeginOverlap(Sphere)
  (params (OverlappedComponent :type Primitive%20Component%20Object%20Reference) (OtherActor :type Actor%20Object%20Reference) (OtherComp :type Primitive%20Component%20Object%20Reference) (OtherBodyIndex :type Integer) (bFromSweep :type Boolean) (SweepResult :type Hit%20Result%20Structure%20%28by%20ref%29))
  (bind _returnvalue (Actor|GetComponentbyClass OtherActor "/Game/Blueprints/levelGenerator/ObstacleItems/Components/BP_AC_OnMagneet.BP_AC_OnMagneet_C"))
  (Utilities|IsValid _returnvalue
    (:Is%20Valid
      (Default|Start _returnvalue (Variables|Default|GetBoat) (Variables|Settings|GetAcceleration2)))))

(event EventActivate
  (CallFunction|SetRadius (Variables|Settings|GetActivetedRadius))
  (Utilities|Time|ClearandInvalidateTimerbyHandle (Variables|Default|GetTimer))
  (bind _returnvalue (Utilities|Time|SetTimerbyFunctionName 0 "Deactivate" (Variables|Settings|GetDuration)))
  (Variables|Default|SetTimer _returnvalue))

(event EventDeactivate
  (CallFunction|SetRadius (Variables|Settings|GetDeactivatedRadius)))

(fn ConstructionScript
  (CallFunction|Deactivate))

(fn SetRadius
  (params (Radius :type Float%20%28single-precision%29))
  (bind _output_get (Variables|Default|SetCurrentRadius Radius))
  (Components|Sphere|SetSphereRadius (Variables|Default|GetSphere) _output_get true))