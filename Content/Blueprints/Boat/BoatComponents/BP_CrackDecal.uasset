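; BP_CrackDecal is a boat component Blueprint that reveals crack decals one at a time on the left or right side.
; The construction script gathers four components per side into Left and Right arrays.
; RandomCrackLeft and RandomCrackRight each unhide a random entry from their array and remove it, so no crack repeats and calls do nothing once that side is exhausted.
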(fn ConstructionScript
  (Variables|Default|SetLeft (Utilities|Array|MakeArray (Variables|Default|GetLeft0) (Variables|Default|GetLeft1) (Variables|Default|GetLeft2) (Variables|Default|GetLeft3)))
  (Variables|Default|SetRight (Utilities|Array|MakeArray (Variables|Default|GetRight1) (Variables|Default|GetRight2) (Variables|Default|GetRight3) (Variables|Default|GetRigh4))))

(fn RandomCrackLeft
  (bind _left (Variables|Default|GetLeft))
  (if (> (Utilities|Array|Length _left) 0)
    (LocalVariables|SetIndex (Math|Random|RandomIntegerinRange 0 (Utilities|Array|LastIndex _left)))
    (Development|SetHiddeninGame (Utilities|Array|Get(acopy) _left (LocalVariables|GetIndex)) false false)
    (Utilities|Array|RemoveIndex (Variables|Default|GetLeft) (LocalVariables|GetIndex))))

(fn RandomCrackRight
  (bind _right (Variables|Default|GetRight))
  (if (> (Utilities|Array|Length _right) 0)
    (LocalVariables|SetIndex (Math|Random|RandomIntegerinRange 0 (Utilities|Array|LastIndex _right)))
    (Development|SetHiddeninGame (Utilities|Array|Get(acopy) _right (LocalVariables|GetIndex)) false false)
    (Utilities|Array|RemoveIndex _right (LocalVariables|GetIndex))))