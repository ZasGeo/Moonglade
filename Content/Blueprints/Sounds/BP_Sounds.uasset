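; Central sound manager for the VR boat game that registers itself on the player pawn and plays pickup, collision, boost and game-over sounds.
; Tile type changes (Simple, Cave, Canion) adjust reverb, stream, wind and cricket layers.
; A self-rescheduling timer plays random ambient sounds from the current tile's group, offset along Y from the player at type-based heights.
; Music switches by fading on a timeline, swapping tracks, then reversing the timeline.
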(event Custom|Wind
  (CallFunction|SailSound))

(event Custom|PickSmallCollectible
  (Audio|PlaySoundatLocation "/Game/Sounds/Gameplay/Small_Collectible_Pickup.Small_Collectible_Pickup" (Transformation|GetActorLocation (Variables|Default|GetPlayer))))

(event Custom|ChangeTypeOfEnviroment
  (params (Type :type TypeOfEnvironment%20Enum))
  (bind _fx_background_wind (Variables|Components|GetFX_Background_Wind))
  (bind _fx_background_wind_2 (Variables|Components|GetFX_Background_Wind))
  (bind _fx_stream (Variables|Components|GetFX_Stream))
  (bind _fx_stream_2 (Variables|Components|GetFX_Stream))
  (bind _fx_stream_3 (Variables|Components|GetFX_Stream))
  (bind _fx_background_wind_3 (Variables|Components|GetFX_Background_Wind))
  (bind _output_get (Variables|Default|SetCurrentTileType Type))
  (switch Utilities|FlowControl|Switch|SwitchonTypeOfEnvironment _output_get
    (:NewEnumerator0
      (Class|GameplayStatics|DeactivateReverbEffect "None")
      (Audio|Components|Audio|SetSound _fx_stream "/Game/Sounds/Ambient/Main_Flow.Main_Flow")
      (Audio|Components|Audio|Play _fx_stream 0.0)
      (Audio|Components|Audio|SetVolumeMultiplier _fx_stream 1.0 :!class /Script/Engine.AudioComponent)
      (Audio|Components|Audio|SetVolumeMultiplier (Variables|Components|GetFX_Background_Wind) 0.6 :!class /Script/Engine.AudioComponent)
      (Audio|Components|Audio|SetSound _fx_background_wind_3 "/Game/Sounds/Ambient/Main_Wind.Main_Wind")
      (Audio|Components|Audio|Play _fx_background_wind_3 0.0)
      (Components|Activation|Activate (Variables|Components|GetFX_Background_cricjets) false)
      (Utilities|IsValid (Variables|Default|GetCaveFlow)
        (:Is%20Valid
          (Components|DestroyComponent (Variables|Default|GetCaveFlow)))))
    (:NewEnumerator1
      (Class|GameplayStatics|ActivateReverbEffect "/Game/Sounds/FX_ReverbCave.FX_ReverbCave" "None" 0.3 0.5 1.0)
      (Audio|Components|Audio|SetSound _fx_stream_3 "/Game/Sounds/Ambient/Cave_Flow.Cave_Flow")
      (Audio|Components|Audio|Play _fx_stream_3 0.0)
      (Audio|Components|Audio|SetVolumeMultiplier _fx_stream_3 0.3 :!class /Script/Engine.AudioComponent)
      (Audio|Components|Audio|SetSound _fx_background_wind_2 "/Game/Sounds/Ambient/Cave_Wind.Cave_Wind")
      (Audio|Components|Audio|Play _fx_background_wind_2 0.0)
      (bind _returnvalue (Audio|CreateSound2D "/Game/Sounds/Ambient/Cave_Flow.Cave_Flow" 0.5 1.0 0.0 0 false false))
      (bind _output_get_2 (Variables|Default|SetCaveFlow _returnvalue))
      (Audio|Components|Audio|Play _output_get_2 0.0)
      (Components|Activation|Deactivate (Variables|Components|GetFX_Background_cricjets)))
    (:NewEnumerator2
      (Class|GameplayStatics|ActivateReverbEffect "/Game/Sounds/FX_CanionReverb.FX_CanionReverb" "None" 0.3 0.5 1.0)
      (Audio|Components|Audio|SetVolumeMultiplier _fx_stream_2 (* (Variables|/Script/Engine.AudioComponent|GetVolumeMultiplier _fx_stream_2) 1.5) :!class /Script/Engine.AudioComponent)
      (Audio|Components|Audio|SetVolumeMultiplier _fx_background_wind (* (Variables|/Script/Engine.AudioComponent|GetVolumeMultiplier _fx_background_wind) 1.5) :!class /Script/Engine.AudioComponent)
      (CallFunction|SailSound)
      (Components|Activation|Deactivate (Variables|Components|GetFX_Background_cricjets)))))

(event Custom|SwichMusic
  (params (NewSound :type Sound%20Base%20Object%20Reference))
  (bind _fx_music (Variables|Components|GetFX_Music))
  (bind (_direction _newtrack_0) (Timeline|MusicTimer PlayFromStart)
    (:Update
      (Audio|Components|Audio|SetVolumeMultiplier (Variables|Components|GetFX_Music) _newtrack_0 :!class /Script/Engine.AudioComponent))
    (:Finished
      (if (not (Utilities|Select :Index _direction :Forward false :Backward true))
        (Audio|Components|Audio|SetSound _fx_music NewSound)
        (Audio|Components|Audio|Play _fx_music 0.0)
        (Timeline|MusicTimer ReverseFromEnd)))))

(event Custom|SailSound
  (Audio|PlaySound2D "/Game/Sounds/Gameplay/Speed_Booster.Speed_Booster"))

(event Custom|PlayChain
  (Audio|PlaySound2D "/Game/Sounds/Gameplay/Chain_Up.Chain_Up"))

(event Custom|CollisionRock
  (Audio|PlaySoundatLocation (Utilities|Select :Index (Math|Random|RandomIntegerinRange 0 1) :Option%200 "/Game/Sounds/Gameplay/Rock_Collision_1.Rock_Collision_1" :Option%201 "/Game/Sounds/Gameplay/Rock_Collision_2.Rock_Collision_2") (Transformation|GetActorLocation (Variables|Default|GetPlayer))))

(event Custom|CollisionWood
  (Audio|PlaySoundatLocation "/Game/Sounds/Gameplay/Wood_Collision_1.Wood_Collision_1" (Transformation|GetActorLocation (Variables|Default|GetPlayer))))

(event Custom|PickCollectible
  (bind _player (Variables|Default|GetPlayer))
  (Audio|PlaySoundatLocation (Utilities|Select :Index (Math|Random|RandomIntegerinRange 0 4) :Option%200 "/Game/Sounds/Gameplay/Spirit-2.Spirit-2" :Option%201 "/Game/Sounds/Gameplay/Spirit-4.Spirit-4" :Option%202 "/Game/Sounds/Gameplay/Spirit-8.Spirit-8" :Option%203 "/Game/Sounds/Gameplay/Spirit-9.Spirit-9" :Option%204 "/Game/Sounds/Gameplay/Spirit-5.Spirit-5") (Transformation|GetActorLocation (Variables|Default|GetPlayer)) "0, 0, 0" 0.2)
  (Utilities|FlowControl|RetriggerableDelay 0.2)
  (Audio|PlaySoundatLocation (Utilities|Select :Index (- (Variables|/Game/Blueprints/levelGenerator/AutoLVL_GameMode.AutoLVL_GameMode_C|GetScoreMultiply (Variables|/Game/Blueprints/Boat/BP_Pawn_VRBoat.BP_Pawn_VRBoat_C|GetGameMode _player)) 1) :Option%200 "/Game/Sounds/Gameplay/Big_Collectible_Pickup_1.Big_Collectible_Pickup_1" :Option%201 "/Game/Sounds/Gameplay/Big_Collectible_Pickup_2.Big_Collectible_Pickup_2" :Option%202 "/Game/Sounds/Gameplay/Big_Collectible_Pickup_3.Big_Collectible_Pickup_3" :Option%203 "/Game/Sounds/Gameplay/Big_Collectible_Pickup_4.Big_Collectible_Pickup_4" :Option%204 "/Game/Sounds/Gameplay/Big_Collectible_Pickup_5.Big_Collectible_Pickup_5") (Transformation|GetActorLocation _player)))

(event Custom|Arch
  (Audio|PlaySoundatLocation "/Game/Sounds/UI_Sounds/Start_Temp.Start_Temp" (Transformation|GetActorLocation (Variables|Default|GetPlayer))))

(event Custom|GameOver
  (Audio|PlaySound2D "/Game/Sounds/Gameplay/Boat_Crush.Boat_Crush")
  (CallFunction|SwichMusic "/Game/Sounds/Music/Dreamboat_2.Dreamboat_2"))

(event EventBeginPlay
  (bind _asbp_pawn_vrboat (Utilities|Casting|CastToBP_Pawn_VRBoat (Game|Player|GetPlayerPawn 0)))
  (bind _output_get (Variables|Default|SetPlayer _asbp_pawn_vrboat))
  (Variables|/Game/Blueprints/Boat/BP_Pawn_VRBoat.BP_Pawn_VRBoat_C|SetSounds _output_get self)
  (Utilities|Time|SetTimerbyFunctionName 0 "PlayRandomSound" 1e+01)
  (Class|GameplayStatics|ActivateReverbEffect "/Game/Sounds/FX_ReverbCave.FX_ReverbCave" "None" 0.3 0.5 1.0))

(fn ConstructionScript)

(fn PlayRandomSound
  (bind _output_get (LocalVariables|SetL_Group (Utilities|Select :Index (Variables|Default|GetCurrentTileType) :NewEnumerator0 (Variables|Default|GetBackgroundActivity_Simple) :NewEnumerator1 (Variables|Default|GetBackgroundActivity_Cave) :NewEnumerator2 (Variables|Default|GetBackgroundActivity_Canion))))
  (Audio|PlaySoundatLocation (Utilities|Array|Get(acopy) (.A_Sound (Utilities|Struct|BreakST_Sound_Types (Utilities|Array|Get(acopy) (.Sounds (Utilities|Struct|BreakSt_Sound_Groups _output_get)) (Math|Random|RandomIntegerinRange 0 (Utilities|Array|LastIndex (.Sounds (Utilities|Struct|BreakSt_Sound_Groups _output_get))))))) (Math|Random|RandomIntegerinRange 0 (Utilities|Array|LastIndex (.A_Sound (Utilities|Struct|BreakST_Sound_Types (Utilities|Array|Get(acopy) (.Sounds (Utilities|Struct|BreakSt_Sound_Groups _output_get)) (Math|Random|RandomIntegerinRange 0 (Utilities|Array|LastIndex (.Sounds (Utilities|Struct|BreakSt_Sound_Groups _output_get)))))))))) (CallFunction|GetSoundLocation (.Type (Utilities|Struct|BreakST_Sound_Types (Utilities|Array|Get(acopy) (.Sounds (Utilities|Struct|BreakSt_Sound_Groups _output_get)) (Math|Random|RandomIntegerinRange 0 (Utilities|Array|LastIndex (.Sounds (Utilities|Struct|BreakSt_Sound_Groups _output_get)))))))) "0, 0, 0" 2.0 1.0 0.0 (.Attenuation (Utilities|Struct|BreakSt_Sound_Groups _output_get)))
  (Utilities|Time|SetTimerbyFunctionName 0 "PlayRandomSound" (Math|Random|RandomFloatinRange 1e+01 2e+01)))

(fn GetSoundLocation
  (params (Type :type E_TypeOfSound%20Enum))
  (return (Math|Vector|MakeVector (Math|Random|RandomFloatinRange -3.6e+03 3.6e+03) (+ (.y (Transformation|GetActorLocation (Variables|Default|GetPlayer))) (Math|Random|RandomFloatinRange 5e+02 1.5e+03)) (Utilities|Select :Index Type :NewEnumerator0 0.0 :NewEnumerator1 5e+02 :NewEnumerator2 8e+02 :NewEnumerator3 0.0))))