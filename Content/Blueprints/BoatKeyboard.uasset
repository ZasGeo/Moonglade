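; Boat actor that moves a fixed +Y offset every tick, with mouse-driven camera rotation.
; Q, E and Space adjust or toggle SpeedMult, but movement ignores it.
; The construction script bends a spline mesh between Start and End, and AddColl counts collectibles.
; Staged destruction, distance scoring, lamp and light ramps, and setup for the decal-cycling timer are all disconnected.
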(event EventBeginPlay)

(event EventTick
  (params (DeltaSeconds :type Float%20%28single-precision%29))
  (Transformation|AddActorWorldOffset "0,150.000000, 0"))

(event Input|MouseEvents|MouseX
  (params (AxisValue :type Float%20%28single-precision%29))
  (Transformation|AddRelativeRotation (Variables|Default|GetCamera) (Math|Rotator|MakeRotator 0.0 0.0 AxisValue) false false))

(event Input|MouseEvents|MouseY
  (params (AxisValue :type Float%20%28single-precision%29))
  (Transformation|AddRelativeRotation (Variables|Default|GetCamera) (Math|Rotator|MakeRotator 0.0 AxisValue 0.0) false false))

(event Input|KeyboardEvents|SpaceBar
  (params (Key :type Key%20Structure :default "AnyKey"))
  (:Pressed
    (Utilities|FlowControl|FlipFlop
      (:A
        (Variables|Default|SetSpeedMult 0))
      (:B
        (Variables|Default|SetSpeedMult (Variables|Default|GetDefaultSpeedMult))))))

(event Input|KeyboardEvents|Q
  (params (Key :type Key%20Structure :default "AnyKey"))
  (:Pressed
    (bind _output_get (Variables|Default|SetSpeedMult (+ (Variables|Default|GetSpeedMult) -10)))
    (Variables|Default|SetDefaultSpeedMult _output_get)))

(event Input|KeyboardEvents|E
  (params (Key :type Key%20Structure :default "AnyKey"))
  (:Pressed
    (bind _output_get (Variables|Default|SetSpeedMult (+ (Variables|Default|GetSpeedMult) 10)))
    (Variables|Default|SetDefaultSpeedMult _output_get)))

(fn ConstructionScript
  (bind _start (Variables|Default|GetStart))
  (bind _end (Variables|Default|GetEnd))
  (bind _returnvalue (Transformation|GetRelativeTransform _end))
  (bind _returnvalue_2 (Transformation|GetRelativeTransform _start))
  (bind (_location _rotation _scale) (Math|Transform|BreakTransform _returnvalue_2))
  (bind (_location_2 _rotation_2 _scale_2) (Math|Transform|BreakTransform _returnvalue))
  (bind _returnvalue_3 (- _location _location_2))
  (bind _returnvalue_4 (Math|Vector|VectorLength _returnvalue_3))
  (SplineMesh|SetStartandEnd (Variables|Default|GetSplineMesh) _location (* (* (Math|Vector|GetForwardVector _rotation) _scale) _returnvalue_4) _location_2 (* (* (Math|Vector|GetForwardVector _rotation_2) _scale_2) _returnvalue_4) true :!class /Script/Engine.SplineMeshComponent))

(fn AddColl
  (Math|Integer|IncrementInt (Variables|Default|GetCollectibles)
    (:%20%20
      (Utilities|Casting|CastToW_SCores (UserInterface|GetUserWidgetObject (Variables|Default|GetWidget))))))

(fn Tmp
  (bind _decal_1st (Variables|Default|GetDecal_1st))
  (bind _returnvalue (Rendering|Material|GetScalarParameterValue _decal_1st "Value /10" :!class /Script/Engine.MaterialInstanceDynamic))
  (Rendering|Material|SetScalarParameterValue _decal_1st "Value /10" (select (>= (+ _returnvalue 0.1) 0.91) 0.0 (+ _returnvalue 0.1)) :!class /Script/Engine.MaterialInstanceDynamic))