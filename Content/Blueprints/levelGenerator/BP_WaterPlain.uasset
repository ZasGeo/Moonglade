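; Water plain actor for the level generator that shifts its two trigger boxes along Y as the player's boat passes, apparently to keep the water going.
; On BeginPlay it stores the absolute Y distance between Box and Box1.
; When a VR or keyboard boat overlaps either box, the other box moves by that distance in +Y.
; The overlapped box briefly disables its collision to avoid immediate retriggering.
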(event OnComponentBeginOverlap(Box)
  (params (OverlappedComponent :type Primitive%20Component%20Object%20Reference) (OtherActor :type Actor%20Object%20Reference) (OtherComp :type Primitive%20Component%20Object%20Reference) (OtherBodyIndex :type Integer) (bFromSweep :type Boolean) (SweepResult :type Hit%20Result%20Structure%20%28by%20ref%29))
  (Utilities|Casting|CastToBP_Pawn_VRBoat OtherActor
    (:then
      _)
    (:CastFailed
      (Utilities|Casting|CastToBoatKeyboard OtherActor)))
  (Collision|SetCollisionEnabled (Variables|Default|GetBox) "NoCollision")
  (Transformation|AddWorldOffset (Variables|Default|GetBox1) (Math|Vector|MakeVector 0.0 (Variables|Default|GetDistanceToTeleport) 0.0) false false)
  (Utilities|FlowControl|Delay 2.0)
  (Collision|SetCollisionEnabled (Variables|Default|GetBox) "QueryOnly"))

(event OnComponentBeginOverlap(Box1)
  (params (OverlappedComponent :type Primitive%20Component%20Object%20Reference) (OtherActor :type Actor%20Object%20Reference) (OtherComp :type Primitive%20Component%20Object%20Reference) (OtherBodyIndex :type Integer) (bFromSweep :type Boolean) (SweepResult :type Hit%20Result%20Structure%20%28by%20ref%29))
  (Utilities|Casting|CastToBP_Pawn_VRBoat OtherActor
    (:then
      _)
    (:CastFailed
      (Utilities|Casting|CastToBoatKeyboard OtherActor)))
  (Collision|SetCollisionEnabled (Variables|Default|GetBox1) "NoCollision")
  (Transformation|AddWorldOffset (Variables|Default|GetBox) (Math|Vector|MakeVector 0.0 (Variables|Default|GetDistanceToTeleport) 0.0) false false)
  (Utilities|FlowControl|Delay 2.0)
  (Collision|SetCollisionEnabled (Variables|Default|GetBox1) "QueryOnly"))

(event EventBeginPlay
  (Variables|Default|SetDistanceToTeleport (Math|Float|Absolute(Float) (- (.y (Transformation|GetWorldLocation (Variables|Default|GetBox1))) (.y (Transformation|GetWorldLocation (Variables|Default|GetBox)))))))

(fn ConstructionScript)