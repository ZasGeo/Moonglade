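; BP_StartZone is the level generator's start tile for the VR boat, publishing its EndPoint as the game mode's tile spawn location.
; When the boat overlaps TileEnd, it starts the easy level, requests a new tile and changes environment sound.
; After a delay, Deactivate disables collision, hides start objects and enables Tick, which tilts and sinks the tile pivot.
; Activate restores the pivot, collision and visibility for reuse.
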(event OnComponentBeginOverlap(TileEnd)
  (params (OverlappedComponent :type Primitive%20Component%20Object%20Reference) (OtherActor :type Actor%20Object%20Reference) (OtherComp :type Primitive%20Component%20Object%20Reference) (OtherBodyIndex :type Integer) (bFromSweep :type Boolean) (SweepResult :type Hit%20Result%20Structure%20%28by%20ref%29))
  (bind _asbp_pawn_vrboat (Utilities|Casting|CastToBP_Pawn_VRBoat OtherActor))
  (Default|Gain _asbp_pawn_vrboat 1.0)
  (Default|StartEasyLvl _asbp_pawn_vrboat)
  (Collision|SetCollisionEnabled (Variables|Default|GetTileEnd) "NoCollision")
  (Default|AddTilePlane (Variables|Default|GetGameMode))
  (Default|ChangeTypeOfEnviroment (Variables|/Game/Blueprints/Boat/BP_Pawn_VRBoat.BP_Pawn_VRBoat_C|GetSounds _asbp_pawn_vrboat) "NewEnumerator0")
  (Utilities|FlowControl|Delay 15.0)
  (CallFunction|Deactivate))

(event EventBeginPlay
  (bind _asauto_lvl_game_mode (Utilities|Casting|CastToAutoLVL_GameMode (Game|GetGameMode)))
  (bind _output_get (Variables|Default|SetGameMode _asauto_lvl_game_mode))
  (Variables|/Game/Blueprints/levelGenerator/AutoLVL_GameMode.AutoLVL_GameMode_C|SetSpawnTLocation _output_get (Transformation|GetWorldLocation (Variables|Default|GetEndPoint)))
  (Variables|Default|SetPointDefaultLocation (Variables|/Script/Engine.SceneComponent|GetRelativeLocation (Variables|Default|GetTileRotatePointDown))))

(event EventTick
  (params (DeltaSeconds :type Float%20%28single-precision%29))
  (bind _output_get (Variables|Default|SetAlphaRot (Math|Float|Clamp(Float) (+ (Variables|Default|GetAlphaRot) (* (Utilities|Time|GetWorldDeltaSeconds) (Variables|Default|GetSpeedRotator_Div))))))
  (if (<= _output_get 0.99)
    (Transformation|SetRelativeRotation (Variables|Default|GetTileRotatePointDown) (Math|Rotator|MakeRotator (Math|Float|Lerp 0.0 -4e+01 (Variables|Default|GetAlphaRot)) 0.0 0.0) false false)
    (elif (>= (.z (Transformation|GetWorldLocation (Variables|Default|GetTileRotatePointDown))) -2.8e+04)
      (Transformation|AddRelativeLocation (Variables|Default|GetTileRotatePointDown) "0, 0,-100.000000" false false)
      (else
        (Rendering|SetActorHiddenInGame false)
        (Actor|Tick|SetActorTickEnabled false)))))

(fn ConstructionScript)

(fn Deactivate
  (Collision|SetActorEnableCollision false)
  (Actor|Tick|SetActorTickEnabled true)
  (for _array_element (Variables|Default|GetStartObjects)
    (Rendering|SetActorHiddenInGame _array_element true)))

(fn Activate
  (bind _tilerotatepointdown (Variables|Default|GetTileRotatePointDown))
  (Actor|Tick|SetActorTickEnabled false)
  (Transformation|SetRelativeRotation _tilerotatepointdown (Math|Rotator|MakeRotator 0.0 0.0 0.0) false false)
  (Transformation|SetRelativeLocation _tilerotatepointdown (Variables|Default|GetPointDefaultLocation) false false)
  (Collision|SetActorEnableCollision true)
  (Rendering|SetActorHiddenInGame false)
  (Collision|SetCollisionEnabled (Variables|Default|GetTileEnd) "QueryOnly")
  (for _array_element (Variables|Default|GetStartObjects)
    (Rendering|SetActorHiddenInGame _array_element false)))