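; BP_Obstacle_Rock is a rock obstacle for the level generator that the VR boat can collide with.
; Init async-loads a random mesh from its Meshes list, applies it and gives the actor a random yaw.
; When BP_Pawn_VRBoat overlaps the mesh, the rock calls the boat's RockColl with its XY location at zero height.
; Its collision switches off on each hit and a one-second timer re-enables it.
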(event OnComponentBeginOverlap(StaticMesh)
  (params (OverlappedComponent :type Primitive%20Component%20Object%20Reference) (OtherActor :type Actor%20Object%20Reference) (OtherComp :type Primitive%20Component%20Object%20Reference) (OtherBodyIndex :type Integer) (bFromSweep :type Boolean) (SweepResult :type Hit%20Result%20Structure%20%28by%20ref%29))
  (bind _asbp_pawn_vrboat (Utilities|Casting|CastToBP_Pawn_VRBoat OtherActor))
  (CallFunction|OnOverlap _asbp_pawn_vrboat))

(event EventInit
  (bind _meshes (Variables|Default|GetMeshes))
  (bind _object (Utilities|AsyncLoadAsset (Utilities|Array|Get(acopy) _meshes (Math|Random|RandomIntegerinRange 0 (Utilities|Array|LastIndex _meshes))))
    (:Completed
      (bind _asstatic_mesh (Utilities|Casting|CastToStaticMesh _object))
      (Components|StaticMesh|SetStaticMesh (Variables|Default|GetStaticMesh) _asstatic_mesh)
      (Transformation|SetActorRotation (Math|Rotator|MakeRotator 0.0 0.0 (Math|Random|RandomFloatinRange 0.0 3.6e+02))))))

(event EventEnable
  (Collision|SetActorEnableCollision true))

(event EventDisable
  (Collision|SetActorEnableCollision false))

(fn ConstructionScript)

(fn OnOverlap
  (params (Actor :type BP%20Pawn%20VR%20Boat%20Object%20Reference))
  (bind _returnvalue (Transformation|GetActorLocation))
  (CallFunction|Disable)
  (Default|RockColl Actor (Math|Vector|MakeVector (.x _returnvalue) (.y _returnvalue) 0.0))
  (CallFunction|Reset)
  (return false))

(fn GetMesh
  (return (Variables|Default|GetStaticMesh)))

(fn Reset
  (Utilities|Time|SetTimerbyFunctionName 0 "Enable" 1.0))