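; Level-generator item, named as a double small collectible, that spins two spheres around the actor's origin.
; The construction script offsets the spheres in opposite directions along a normalized Axis by Radius.
; Tick accumulates an angle from Speed and sets absolute rotation about the perpendicular to Axis nearest world up, found by double cross product.
; Activate resets the angle, unhides and enables tick; Deactivate hides and stops tick, allowing reuse.
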(event EventTick
  (params (DeltaSeconds :type Float%20%28single-precision%29))
  (bind _axis (Variables|Default|GetAxis))
  (bind _returnvalue (Math|Vector|Normalize _axis))
  (Variables|Default|SetRot (+ (Variables|Default|GetRot) (* DeltaSeconds (Variables|Default|GetSpeed))))
  (Transformation|SetActorRotation (Math|Vector|RotatorfromAxisandAngle (Math|Vector|CrossProduct (Math|Vector|CrossProduct _returnvalue "0, 0,1.000000") _returnvalue) (Variables|Default|GetRot))))

(fn ConstructionScript
  (bind _axis (Variables|Default|GetAxis))
  (bind _returnvalue (Math|Vector|Normalize _axis))
  (Transformation|AddLocalOffset (Variables|Default|GetSphere) (* _returnvalue (Variables|Default|GetRadius)) false false)
  (Transformation|AddLocalOffset (Variables|Default|GetSphere1) (* _returnvalue (* (Variables|Default|GetRadius) -1.0)) false false))

(fn Activate
  (Variables|Default|SetRot 0.0)
  (Rendering|SetActorHiddenInGame false)
  (Actor|Tick|SetActorTickEnabled true))

(fn Deactivate
  (Rendering|SetActorHiddenInGame true)
  (Actor|Tick|SetActorTickEnabled false))