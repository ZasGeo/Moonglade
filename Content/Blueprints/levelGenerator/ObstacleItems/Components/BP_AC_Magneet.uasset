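; Magnet component for level-generator obstacle items that pulls its owning actor toward the boat's Lamp.
; Start stores the boat and acceleration increment and enables Tick, which compounds acceleration and speed per frame, without delta time, while adding boat motion.
; Within DistanceToStop, Stop disables Tick and schedules Reset after a delay interpolated by boat speed.
; Reset returns the owner to zero relative location and clears speed and acceleration.
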(event EventBeginPlay
  (Variables|Default|SetOwner (Components|GetOwner)))

(event EventTick
  (params (DeltaSeconds :type Float%20%28single-precision%29))
  (bind _boat (Variables|Default|GetBoat))
  (bind _owner (Variables|Default|GetOwner))
  (bind _boat_2 (Variables|Default|GetBoat))
  (bind _returnvalue (Transformation|GetActorLocation _owner))
  (bind _lamp (Variables|/Game/Blueprints/Boat/BP_Pawn_VRBoat.BP_Pawn_VRBoat_C|GetLamp _boat))
  (bind _returnvalue_2 (Transformation|GetWorldLocation _lamp))
  (bind _returnvalue_3 (- _returnvalue_2 _returnvalue))
  (Variables|Default|SetAcceleration (+ (Variables|Default|GetAcceleration) (Variables|Default|GetAcceleration2)))
  (Variables|Default|SetSpeed (+ (Variables|Default|GetSpeed) (Variables|Default|GetAcceleration)))
  (if (<= (Math|Vector|VectorLength _returnvalue_3) (Variables|Default|GetDistanceToStop))
    (CallFunction|Stop)
    (else
      (Transformation|SetActorLocation (Variables|Default|GetOwner) (+ _returnvalue (+ (Math|Vector|MakeVector (* (.x (Math|Vector|GetForwardVector (Variables|/Game/Blueprints/Boat/BP_Pawn_VRBoat.BP_Pawn_VRBoat_C|GetArrow _boat_2))) (Variables|/Game/Blueprints/Boat/BP_Pawn_VRBoat.BP_Pawn_VRBoat_C|GetSpeed _boat_2)) (Variables|/Game/Blueprints/Boat/BP_Pawn_VRBoat.BP_Pawn_VRBoat_C|GetSpeed _boat_2) 0.0) (* (Math|Vector|Normalize _returnvalue_3) (Variables|Default|GetSpeed)))) false false))))

(fn Start
  (params (Boat :type BP%20Pawn%20VR%20Boat%20Object%20Reference) (Acceleration :type Float%20%28single-precision%29))
  (Variables|Default|SetAcceleration2 Acceleration)
  (Variables|Default|SetBoat Boat)
  (Components|Tick|SetComponentTickEnabled true))

(fn Stop
  (bind _boat (Variables|Default|GetBoat))
  (bind _resettime (Variables|Default|GetResetTime))
  (bind _speed (Variables|/Game/Blueprints/Boat/BP_Pawn_VRBoat.BP_Pawn_VRBoat_C|GetSpeed _boat))
  (bind _maxspeed (Variables|/Game/Blueprints/Boat/BP_Pawn_VRBoat.BP_Pawn_VRBoat_C|GetMaxSpeed _boat))
  (bind _returnvalue (- _maxspeed _speed))
  (bind _returnvalue_2 (/ _returnvalue _maxspeed))
  (bind _returnvalue_3 (Math|Float|Clamp(Float) _returnvalue_2))
  (bind _returnvalue_4 (Math|Float|Lerp 2.0 _resettime _returnvalue_3))
  (Development|PrintString (Utilities|String|ToString(Float) _returnvalue_4))
  (Components|Tick|SetComponentTickEnabled false)
  (Utilities|Time|SetTimerbyFunctionName 0 "Reset" _returnvalue_4)
  (return _returnvalue_4))

(fn Reset
  (Development|PrintString "reset")
  (Transformation|SetActorRelativeLocation (Variables|Default|GetOwner))
  (Variables|Default|SetSpeed 0.0)
  (Variables|Default|SetAcceleration 0.0))