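; Pooled arch obstacle for the level generator that awards score when the VR boat passes through it.
; Activate teleports it to an offset location, reveals it after a delay and removes it from the GameMode's Arches pool.
; Tick lerps roll by UpDownTruefals: upright with collision enabled, or tipped over, hidden far below and re-pooled.
; Boat overlap plays a sound, adds score, disables collision and starts the delayed tip-over.
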(event OnComponentBeginOverlap(Box)
  (params (OverlappedComponent :type Primitive%20Component%20Object%20Reference) (OtherActor :type Actor%20Object%20Reference) (OtherComp :type Primitive%20Component%20Object%20Reference) (OtherBodyIndex :type Integer) (bFromSweep :type Boolean) (SweepResult :type Hit%20Result%20Structure%20%28by%20ref%29))
  (bind _gamemode (Variables|Default|GetGameMode))
  (bind _asbp_pawn_vrboat (Utilities|Casting|CastToBP_Pawn_VRBoat OtherActor))
  (Default|Arch (Variables|/Game/Blueprints/Boat/BP_Pawn_VRBoat.BP_Pawn_VRBoat_C|GetSounds _asbp_pawn_vrboat))
  (Variables|/Game/Blueprints/levelGenerator/AutoLVL_GameMode.AutoLVL_GameMode_C|SetTotalScores _gamemode (+ (Variables|/Game/Blueprints/levelGenerator/AutoLVL_GameMode.AutoLVL_GameMode_C|GetTotalScores _gamemode) 1000))
  (Collision|SetActorEnableCollision false)
  (Utilities|FlowControl|Delay 12.0)
  (Variables|Default|SetAlphaRot 0.0)
  (Variables|Default|SetUp/Down-True/fals false)
  (Actor|Tick|SetActorTickEnabled true))

(event Custom|Activate
  (params (Location :type Vector))
  (Transformation|Teleport (Math|Vector|MakeVector (.x Location) (+ (.y Location) 6e+04) 0.0) "0, 0,60.000000")
  (Utilities|FlowControl|Delay 5.0)
  (Rendering|SetActorHiddenInGame false)
  (Actor|Tick|SetActorTickEnabled true)
  (Utilities|Array|RemoveItem (Variables|/Game/Blueprints/levelGenerator/AutoLVL_GameMode.AutoLVL_GameMode_C|GetArches (Variables|Default|GetGameMode)) self))

(event EventBeginPlay
  (bind _asauto_lvl_game_mode (Utilities|Casting|CastToAutoLVL_GameMode (Game|GetGameMode)))
  (Variables|Default|SetGameMode _asauto_lvl_game_mode))

(event EventTick
  (params (DeltaSeconds :type Float%20%28single-precision%29))
  (if (Variables|Default|GetUp/Down-True/fals)
    (bind _output_get (Variables|Default|SetAlphaRot (Math|Float|Clamp(Float) (+ (Variables|Default|GetAlphaRot) (* (Utilities|Time|GetWorldDeltaSeconds) (Variables|Default|GetSpeedRotator_Div))))))
    (if (<= _output_get 0.99)
      (Transformation|SetActorRotation (Math|Rotator|MakeRotator (Math|Float|Lerp 6e+01 0.0 (Variables|Default|GetAlphaRot)) 0.0 0.0))
      (else
        (Variables|Default|SetAlphaRot 0.0)
        (Transformation|SetActorRotation (Math|Rotator|MakeRotator 0.0 0.0 0.0))
        (Collision|SetActorEnableCollision true)
        (Actor|Tick|SetActorTickEnabled false)))
    (else
      (bind _output_get_2 (Variables|Default|SetAlphaRot (Math|Float|Clamp(Float) (+ (Variables|Default|GetAlphaRot) (* (Utilities|Time|GetWorldDeltaSeconds) (Variables|Default|GetSpeedRotator_Div))))))
      (if (<= _output_get_2 0.99)
        (Transformation|SetActorRotation (Math|Rotator|MakeRotator (Math|Float|Lerp 0.0 -9e+01 (Variables|Default|GetAlphaRot)) 0.0 0.0))
        (else
          (Transformation|Teleport "0.0,0.0,-999999.000000" "0, 0,60.000000")
          (Rendering|SetActorHiddenInGame true)
          (Collision|SetActorEnableCollision false)
          (Utilities|Array|Add (Variables|/Game/Blueprints/levelGenerator/AutoLVL_GameMode.AutoLVL_GameMode_C|GetArches (Variables|Default|GetGameMode)) self)
          (Actor|Tick|SetActorTickEnabled false))))))

(fn ConstructionScript)