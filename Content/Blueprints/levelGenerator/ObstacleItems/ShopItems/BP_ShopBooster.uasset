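; Base shop booster pickup for the VR boat game that detects the player's boat through a sphere overlap.
; On BeginPlay it gets the Shop from AutoLVL_GameMode, binds to its restart event, then hides itself with collision disabled.
; Activate and Deactivate toggle visibility and collision together.
; A boat overlap calls OnOverlap, which is empty here.
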(event OnComponentBeginOverlap(Sphere)
  (params (OverlappedComponent :type Primitive%20Component%20Object%20Reference) (OtherActor :type Actor%20Object%20Reference) (OtherComp :type Primitive%20Component%20Object%20Reference) (OtherBodyIndex :type Integer) (bFromSweep :type Boolean) (SweepResult :type Hit%20Result%20Structure%20%28by%20ref%29))
  (bind _asbp_pawn_vrboat (Utilities|Casting|CastToBP_Pawn_VRBoat OtherActor))
  (CallFunction|OnOverlap _asbp_pawn_vrboat))

(event EventBeginPlay
  (bind _asauto_lvl_game_mode (Utilities|Casting|CastToAutoLVL_GameMode (Game|GetGameMode)))
  (Variables|Default|SetShop (Variables|/Game/Blueprints/levelGenerator/AutoLVL_GameMode.AutoLVL_GameMode_C|GetShop _asauto_lvl_game_mode))
  (CallFunction|Bind)
  (CallFunction|Deactivate))

(fn ConstructionScript)

(fn Bind
  (EventDispatchers|BindEventtoRestart (Variables|Default|GetShop) (EventDispatchers|CreateEvent :!event Deactivate)))

(fn Activate
  (Rendering|SetActorHiddenInGame false)
  (Collision|SetActorEnableCollision true))

(fn Deactivate
  (Rendering|SetActorHiddenInGame true)
  (Collision|SetActorEnableCollision false))

(fn OnOverlap
  (params (Boat :type BP%20Pawn%20VR%20Boat%20Object%20Reference)))