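; BP_MagnetObstacle is a shop-linked level-generator obstacle item that gives the overlapping actor a magnet booster.
; On Bind, it runs the parent logic and hooks a delegate to the Shop's BuyBooster1 event.
; On overlap, it runs the parent handler, activates the actor's Magnet, disables itself and sets a ten-second timer to call Enable.
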(event EventBeginPlay
  (|CallParentFunction))

(event Collision|EventActorBeginOverlap
  (params (OtherActor :type Actor%20Object%20Reference)))

(event EventTick
  (params (DeltaSeconds :type Float%20%28single-precision%29)))

(event EventBind
  (|CallParentFunction)
  (EventDispatchers|BindEventtoBuyBooster1 (Variables|Default|GetShop) (EventDispatchers|CreateEvent :!event Enable)))

(fn ConstructionScript
  (|CallParentFunction))

(fn OnOverlap
  (params (Actor :type BP%20Pawn%20VR%20Boat%20Object%20Reference))
  (bind _huy (|CallParentFunction Actor))
  (Default|Activate (Variables|/Game/Blueprints/Boat/BP_Pawn_VRBoat.BP_Pawn_VRBoat_C|GetMagnet Actor))
  (CallFunction|Disable)
  (Utilities|Time|SetTimerbyFunctionName 0 "Enable" 1e+01)
  (return _huy))