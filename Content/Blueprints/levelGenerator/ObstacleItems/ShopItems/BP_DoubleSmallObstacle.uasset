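; BP_DoubleSmallObstacle is a shop-linked obstacle item in the level generator that activates a double-collectible booster when overlapped.
; BeginPlay caches the first BP_SpecialniyBliadKostylDliaDuubleCol actor found in the level as Kostyl, a workaround helper that receives the activation call.
; Bind hooks into the Shop's Booster1 purchase event.
; On overlap it runs the parent logic, triggers the helper, disables itself and re-enables after a ten-second timer.
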(event EventBeginPlay
  (|CallParentFunction)
  (bind _outactors (Actor|GetAllActorsOfClass "/Game/Blueprints/levelGenerator/ObstacleItems/ShopItems/BP_SpecialniyBliadKostylDliaDuubleCol.BP_SpecialniyBliadKostylDliaDuubleCol_C"))
  (Variables|Default|SetKostyl (Utilities|Array|Get(acopy) _outactors)))

(event EventBind
  (|CallParentFunction)
  (EventDispatchers|BindEventtoBuyBooster1 (Variables|Default|GetShop) (EventDispatchers|CreateEvent :!event Enable)))

(fn ConstructionScript
  (|CallParentFunction))

(fn OnOverlap
  (params (Actor :type BP%20Pawn%20VR%20Boat%20Object%20Reference))
  (bind _huy (|CallParentFunction Actor))
  (Default|DoubbleCollectibleActivate (Variables|Default|GetKostyl))
  (CallFunction|Disable)
  (Utilities|Time|SetTimerbyFunctionName 0 "Enable" 1e+01)
  (return _huy))