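; BP_ShopBuster is a level-generator shop item actor that can be switched on and off by toggling its visibility and collision.
; On BeginPlay it gets the Shop from AutoLVL_GameMode, binds an event to the Shop's restart, then deactivates itself so it starts hidden.
; Activate shows the actor and enables collision, while Deactivate reverses both, leaving the actor in place.
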(event EventBeginPlay
  (bind _asauto_lvl_game_mode (Utilities|Casting|CastToAutoLVL_GameMode (Game|GetGameMode)))
  (Variables|Default|SetShop (Variables|/Game/Blueprints/levelGenerator/AutoLVL_GameMode.AutoLVL_GameMode_C|GetShop _asauto_lvl_game_mode))
  (CallFunction|Bind)
  (CallFunction|Deactivate))

(fn ConstructionScript)

(fn Bind
  (EventDispatchers|BindEventtoRestart (Variables|Default|GetShop) (EventDispatchers|CreateEvent :!event Deactivate)))

(fn Activate
  (Rendering|SetActorHiddenInGame false)
  (Collision|SetActorEnableCollision true))

(fn Deactivate
  (Rendering|SetActorHiddenInGame true)
  (Collision|SetActorEnableCollision false))