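; BP_ObstacleItem is a skeleton obstacle item for the level generator, apparently meant as a base class for specific obstacles.
; BeginPlay calls Init, which calls an empty Bind hook.
; Enable and Disable toggle the actor's visibility and collision together instead of spawning or destroying it.
; OnOverlap returns false and GetMesh returns nothing, leaving both as stubs.
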(event EventBeginPlay
  (CallFunction|Init))

(fn ConstructionScript)

(fn Bind)

(fn Enable
  (Rendering|SetActorHiddenInGame false)
  (Collision|SetActorEnableCollision true))

(fn Disable
  (Rendering|SetActorHiddenInGame true)
  (Collision|SetActorEnableCollision false))

(fn OnOverlap
  (params (Actor :type BP%20Pawn%20VR%20Boat%20Object%20Reference))
  (return false))

(fn Init
  (CallFunction|Bind))

(fn GetMesh
  (return 0))