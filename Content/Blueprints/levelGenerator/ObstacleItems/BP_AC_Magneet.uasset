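; Magnet component for level-generator obstacle items that pulls its owning actor toward the boat's lamp.
; Start caches the boat and original location, then enables Tick, which moves the owner with growing speed plus an offset from boat speed.
; Stop disables Tick and schedules Reset to restore that location, with a delay interpolated from boat speed.
; The distance check that would call Stop is disconnected.
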(event EventBeginPlay
  (Variables|Default|SetOwner (Components|GetOwner))
  (Components|Tick|SetComponentTickEnabled false))

(event EventTick
  (params (DeltaSeconds :type Float%20%28single-precision%29))
  (bind _owner (Variables|Default|GetOwner))
  (bind _boat (Variables|Default|GetBoat))
  (bind _returnvalue (Transformation|GetActorLocation _owner))
  (Variables|Default|SetSpeed (+ (Variables|Default|GetSpeed) (Variables|Default|GetAcceleration)))
  (Transformation|SetActorLocation (Variables|Default|GetOwner) (+ _returnvalue (+ (Math|Vector|MakeVector (* (Variables|/Game/Blueprints/Boat/BP_Pawn_VRBoat.BP_Pawn_VRBoat_C|GetSpeed _boat) (.x (Math|Vector|GetForwardVector (Variables|/Game/Blueprints/Boat/BP_Pawn_VRBoat.BP_Pawn_VRBoat_C|GetArrow _boat)))) (Variables|/Game/Blueprints/Boat/BP_Pawn_VRBoat.BP_Pawn_VRBoat_C|GetSpeed _boat) 0.0) (* (Math|Vector|Normalize (- (Transformation|GetWorldLocation (Variables|/Game/Blueprints/Boat/BP_Pawn_VRBoat.BP_Pawn_VRBoat_C|GetLamp (Variables|Default|GetBoat))) _returnvalue)) (Variables|Default|GetSpeed)))) false false))

(fn Start
  (params (Boat :type BP%20Pawn%20VR%20Boat%20Object%20Reference))
  (Variables|Default|SetBoat Boat)
  (Variables|Default|SetResetLoc (Transformation|GetActorLocation (Variables|Default|GetOwner)))
  (Components|Tick|SetComponentTickEnabled true))

(fn Stop
  (bind _boat (Variables|Default|GetBoat))
  (bind _resettime (Variables|Default|GetResetTime))
  (bind _speed (Variables|/Game/Blueprints/Boat/BP_Pawn_VRBoat.BP_Pawn_VRBoat_C|GetSpeed _boat))
  (bind _maxspeed (Variables|/Game/Blueprints/Boat/BP_Pawn_VRBoat.BP_Pawn_VRBoat_C|GetMaxSpeed _boat))
  (bind _returnvalue (- _maxspeed _speed))
  (bind _returnvalue_2 (/ _returnvalue _maxspeed))
  (bind _returnvalue_3 (Math|Float|Clamp(Float) _returnvalue_2))
  (bind _returnvalue_4 (Math|Float|Lerp 2.0 _resettime _returnvalue_3))
  (Development|PrintString (Utilities|String|ToString(Float) _returnvalue_4))
  (Components|Tick|SetComponentTickEnabled false)
  (Utilities|Time|SetTimerbyFunctionName 0 "Reset" _returnvalue_4)
  (return _returnvalue_4))

(fn Reset
  (Development|PrintString "reset")
  (Transformation|SetActorLocation (Variables|Default|GetOwner) (Variables|Default|GetResetLoc) false false))