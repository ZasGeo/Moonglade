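; Small collectible for the VR boat level generator that notifies the boat pawn when it overlaps the box.
; The mesh gets a random per-axis scale at BeginPlay.
; On pickup, collision turns off and a timeline shrinks the mesh to zero, lerping all axes from its current X scale.
; It then stops its magnet component, waits the returned duration, and restores visibility, collision and starting scale for reuse.
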(event OnComponentBeginOverlap(Box)
  (params (OverlappedComponent :type Primitive%20Component%20Object%20Reference) (OtherActor :type Actor%20Object%20Reference) (OtherComp :type Primitive%20Component%20Object%20Reference) (OtherBodyIndex :type Integer) (bFromSweep :type Boolean) (SweepResult :type Hit%20Result%20Structure%20%28by%20ref%29))
  (bind _staticmesh (Variables|Default|GetStaticMesh))
  (bind _asbp_pawn_vrboat (Utilities|Casting|CastToBP_Pawn_VRBoat OtherActor))
  (Default|SmallCollectible _asbp_pawn_vrboat)
  (Collision|SetCollisionEnabled (Variables|Default|GetBox) "NoCollision")
  (bind _alphascale (Timeline|Scale PlayFromStart)
    (:Update
      (Transformation|SetWorldScale3D _staticmesh (Math|Vector|MakeVector (Math|Float|Lerp (.x (Transformation|GetWorldScale _staticmesh)) 0.0 _alphascale) (Math|Float|Lerp (.x (Transformation|GetWorldScale _staticmesh)) 0.0 _alphascale) (Math|Float|Lerp (.x (Transformation|GetWorldScale _staticmesh)) 0.0 _alphascale))))
    (:Finished
      (bind _returnvalue (Default|Stop (Variables|Default|GetBP_AC_Magnet)))
      (Utilities|FlowControl|Delay _returnvalue)
      (Rendering|SetActorHiddenInGame false)
      (Collision|SetCollisionEnabled (Variables|Default|GetBox) "QueryOnly")
      (Transformation|SetRelativeScale3D (Variables|Default|GetStaticMesh) (Variables|Default|GetStartScale)))))

(event EventBeginPlay
  (bind _returnvalue (Math|Random|RandomFloatinRange 0.8 1.2))
  (bind _output_get (Variables|Default|SetStartScale (Math|Vector|MakeVector _returnvalue _returnvalue _returnvalue)))
  (Transformation|SetRelativeScale3D (Variables|Default|GetStaticMesh) _output_get))

(fn ConstructionScript)