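; Floating wood obstacle in the level generator that gets knocked aside by the VR boat.
; On BeginPlay it async-loads a random mesh, randomizes yaw and runs its timeline once.
; Boat overlap disables collision, calls the boat's WoodColl and replays the timeline, pushing the mesh horizontally away with a roll/pitch wobble.
; After a delay, collision, tilt and mesh position reset, a step the author flags for rework.
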(event OnComponentBeginOverlap(StaticMesh)
  (params (OverlappedComponent :type Primitive%20Component%20Object%20Reference) (OtherActor :type Actor%20Object%20Reference) (OtherComp :type Primitive%20Component%20Object%20Reference) (OtherBodyIndex :type Integer) (bFromSweep :type Boolean) (SweepResult :type Hit%20Result%20Structure%20%28by%20ref%29))
  (bind _staticmesh (Variables|Default|GetStaticMesh))
  (bind _returnvalue (Transformation|GetWorldLocation _staticmesh))
  (bind _asbp_pawn_vrboat (Utilities|Casting|CastToBP_Pawn_VRBoat OtherActor))
  (Collision|SetActorEnableCollision false)
  (Variables|Default|SetDirection (Math|Vector|Normalize (Math|Vector|MakeVector (.x (- _returnvalue (Transformation|GetWorldLocation (Variables|/Game/Blueprints/Boat/BP_Pawn_VRBoat.BP_Pawn_VRBoat_C|GetBoatRoot _asbp_pawn_vrboat)))) (.y (- _returnvalue (Transformation|GetWorldLocation (Variables|/Game/Blueprints/Boat/BP_Pawn_VRBoat.BP_Pawn_VRBoat_C|GetBoatRoot _asbp_pawn_vrboat)))) 0.0)))
  (Default|WoodColl _asbp_pawn_vrboat _returnvalue)
  (bind (_direction _force _alpharot) (Timeline|Timeline_0 PlayFromStart)
    (:Update
      (Transformation|AddWorldOffset (Variables|Default|GetStaticMesh) (* (Variables|Default|GetDirection) _force) false false)
      (Transformation|SetActorRotation (Math|Rotator|MakeRotator (Math|Float|Lerp -8.0 8.0 _alpharot) (Math|Float|Lerp -8.0 8.0 _alpharot) (.yaw (Transformation|GetActorRotation)))))
    (:Finished
      ;[1 1 1] huynia. peredelat'
      (Utilities|FlowControl|Delay 5.0)
      (Collision|SetActorEnableCollision true)
      (Transformation|SetActorRotation (Math|Rotator|MakeRotator 0.0 0.0 (.yaw (Transformation|GetActorRotation))))
      (Transformation|SetRelativeLocation (Variables|Default|GetStaticMesh) "0, 0, 0" false false))))

(event EventBeginPlay
  (bind _meshes (Variables|Default|GetMeshes))
  (bind _object (Utilities|AsyncLoadAsset (Utilities|Array|Get(acopy) _meshes (Math|Random|RandomIntegerinRange 0 (Utilities|Array|LastIndex _meshes)))))
  (bind _asstatic_mesh (Utilities|Casting|CastToStaticMesh _object))
  (Components|StaticMesh|SetStaticMesh (Variables|Default|GetStaticMesh) _asstatic_mesh)
  (Transformation|SetActorRotation (Math|Rotator|MakeRotator 0.0 0.0 (Math|Random|RandomFloatinRange -45.0 45.0)))
  (bind (_direction _force _alpharot) (Timeline|Timeline_0 PlayFromStart)
    (:Update
      (Transformation|AddWorldOffset (Variables|Default|GetStaticMesh) (* (Variables|Default|GetDirection) _force) false false)
      (Transformation|SetActorRotation (Math|Rotator|MakeRotator (Math|Float|Lerp -8.0 8.0 _alpharot) (Math|Float|Lerp -8.0 8.0 _alpharot) (.yaw (Transformation|GetActorRotation)))))
    (:Finished
      ;[1 1 1] huynia. peredelat'
      (Utilities|FlowControl|Delay 5.0)
      (Collision|SetActorEnableCollision true)
      (Transformation|SetActorRotation (Math|Rotator|MakeRotator 0.0 0.0 (.yaw (Transformation|GetActorRotation))))
      (Transformation|SetRelativeLocation (Variables|Default|GetStaticMesh) "0, 0, 0" false false))))

(fn ConstructionScript)