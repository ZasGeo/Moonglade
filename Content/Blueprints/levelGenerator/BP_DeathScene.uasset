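; BP_DeathScene is the scene the VR player is teleported to on death, presenting stats and a restart option.
; On Teleported, it switches both of the player's controllers to interaction mode.
; It finds the BP_Restart child actor, refreshes its W_SCores widget with stats, and after a five-second delay calls Act on that restart actor.
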(event Custom|Teleported
  (params (Player :type BP%20Pawn%20VR%20Boat%20Object%20Reference))
  (bind _output_get (Variables|Default|SetPlayer Player))
  (Default|SetInteractionMod (Variables|/Game/Blueprints/Boat/BP_Pawn_VRBoat.BP_Pawn_VRBoat_C|GetLeftController _output_get))
  (bind _asbp_restart (Utilities|Casting|CastToBP_Restart (Variables|/Script/Engine.ChildActorComponent|GetChildActor (Variables|Default|GetChildActor))))
  (bind _asw_scores (Utilities|Casting|CastToW_SCores (UserInterface|GetUserWidgetObject (Variables|/Game/Blueprints/InteractObjects/BP_Restart.BP_Restart_C|GetWidget _asbp_restart))))
  (Default|SetStats _asw_scores)
  (Utilities|FlowControl|Delay 5.0)
  (Default|Act _asbp_restart))

(fn ConstructionScript)