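; Game mode for an endless VR boat level that builds the course from random tiles and scores distance travelled along Y.
; BeginPlay pre-spawns hidden pools of environment tiles, obstacle sets and arches, which are teleported into place instead of spawned at runtime.
; AddTilePlane escalates difficulty by tile count, elapsed time and a MegaCanion transition, mixing in special tiles and arches.
; Cave and canyon obstacle pools are spawned but left unwired in selection.
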(event Custom|StartTimer
  (bind _returnvalue (Utilities|Time|GetGameTimeinSeconds))
  (Utilities|FlowControl|DoOnce false
    (:Completed
      (Variables|Default|SetTimeStart3dDiff _returnvalue)
      (Variables|Default|SetTimeEnd3dDiff (+ _returnvalue (Variables|Default|GetSecondsTo4thDiff))))))

(event EventBeginPlay
  (bind _asbp_pawn_vrboat (Utilities|Casting|CastToBP_Pawn_VRBoat (Game|Player|GetPlayerPawn 0))
    (:then
      (Variables|Default|SetPawn _asbp_pawn_vrboat))
    (:CastFailed
      _))
  (for _array_element (Variables|EnviromentTiles|GetTilesWithEnviromnent)
    (bind _returnvalue (Game|SpawnActorfromClass _array_element (Math|Transform|MakeTransform "-999999.000000, 0,0.000000" "0, 0, 0" "1,1,1") "AlwaysSpawn" 0 0 0))
    (Rendering|SetActorHiddenInGame _returnvalue true)
    (Collision|SetActorEnableCollision _returnvalue false)
    (Utilities|Array|Add (Variables|EnviromentTiles|GetTilesWithEnviromnent_Ref) _returnvalue))
  (for _array_element_2 (Variables|ObstacleTiles|GetObstacleTilesDiff_0)
    (bind _returnvalue_2 (Game|SpawnActorfromClass _array_element_2 (Math|Transform|MakeTransform "-999999.000000, 0,0.000000" "0, 0, 0" "1,1,1") "AlwaysSpawn" 0 0))
    (Rendering|SetActorHiddenInGame _returnvalue_2 true)
    (Collision|SetActorEnableCollision _returnvalue_2 false)
    (Utilities|Array|Add (Variables|ObstacleTiles|GetObstacleTilesDiff_0_Ref) _returnvalue_2))
  (for _array_element_3 (Variables|ObstacleTiles|GetObstacleTilesDiff_1)
    (bind _returnvalue_3 (Game|SpawnActorfromClass _array_element_3 (Math|Transform|MakeTransform "-999999.000000,0.000000,0.000000" "0, 0, 0" "1,1,1") "AlwaysSpawn" 0 0))
    (Rendering|SetActorHiddenInGame _returnvalue_3 true)
    (Collision|SetActorEnableCollision _returnvalue_3 false)
    (Utilities|Array|Add (Variables|ObstacleTiles|GetObstacleTilesDiff_1_Ref) _returnvalue_3))
  (for _array_element_4 (Variables|ObstacleTiles|GetObstacleTilesDiff_2)
    (bind _returnvalue_4 (Game|SpawnActorfromClass _array_element_4 (Math|Transform|MakeTransform "-999999.000000,0.000000,0.000000" "0, 0, 0" "1,1,1") "AlwaysSpawn" 0 0))
    (Rendering|SetActorHiddenInGame _returnvalue_4 true)
    (Collision|SetActorEnableCollision _returnvalue_4 false)
    (Utilities|Array|Add (Variables|ObstacleTiles|GetObstacleTilesDiff_2_Ref) _returnvalue_4))
  (for _array_element_5 (Variables|ObstacleTiles|GetObstacleTilesDiff_3)
    (bind _returnvalue_5 (Game|SpawnActorfromClass _array_element_5 (Math|Transform|MakeTransform "-999999.000000,0.000000,0.000000" "0, 0, 0" "1,1,1") "AlwaysSpawn" 0 0))
    (Rendering|SetActorHiddenInGame _returnvalue_5 true)
    (Collision|SetActorEnableCollision _returnvalue_5 false)
    (Utilities|Array|Add (Variables|ObstacleTiles|GetObstacleTilesDiff_3_Ref) _returnvalue_5))
  (for _array_element_6 (Variables|Default|GetArch_Classes)
    (bind _returnvalue_6 (Game|SpawnActorfromClass _array_element_6 (Math|Transform|MakeTransform "0, 0,-999999.000000" "0, 0, 0" "1,1,1") "AlwaysSpawn" 0 0))
    (Rendering|SetActorHiddenInGame _returnvalue_6 true)
    (Collision|SetActorEnableCollision _returnvalue_6 false)
    (Utilities|Array|Add (Variables|Default|GetArches) _returnvalue_6))
  (for _array_element_7 (Variables|EnviromentTiles|GetTilesWithEnviromnent_Special)
    (bind _returnvalue_7 (Game|SpawnActorfromClass _array_element_7 (Math|Transform|MakeTransform "0, 0,-999999.000000" "0, 0, 0" "1,1,1") "Undefined" 0 0 0))
    (Rendering|SetActorHiddenInGame _returnvalue_7 true)
    (Collision|SetActorEnableCollision _returnvalue_7 false)
    (Utilities|Array|Add (Variables|EnviromentTiles|GetTilesWithEnviromnent_Special_Ref) _returnvalue_7))
  (for _array_element_8 (Variables|Default|GetObstacleTilesDiff_Cave)
    (bind _returnvalue_8 (Game|SpawnActorfromClass _array_element_8 (Math|Transform|MakeTransform "0, 0,-999999.000000" "0, 0, 0" "1,1,1") "Undefined" 0 0))
    (Rendering|SetActorHiddenInGame _returnvalue_8 true)
    (Collision|SetActorEnableCollision _returnvalue_8 false)
    (Utilities|Array|Add (Variables|ObstacleTiles|GetObstacleTilesDiff_Cave_Ref) _returnvalue_8))
  (for _array_element_9 (Variables|Default|GetObstacleTilesDiff_Canion)
    (bind _returnvalue_9 (Game|SpawnActorfromClass _array_element_9 (Math|Transform|MakeTransform "0, 0,-999999.000000" "0, 0, 0" "1,1,1") "Undefined" 0 0))
    (Rendering|SetActorHiddenInGame _returnvalue_9 true)
    (Collision|SetActorEnableCollision _returnvalue_9 false)
    (Utilities|Array|Add (Variables|ObstacleTiles|GetObstacleTilesDiff_Canion_Ref) _returnvalue_9))
  (for _array_element_10 (Variables|ObstacleTiles|GetObstacleTilesDiff_4)
    (bind _returnvalue_10 (Game|SpawnActorfromClass _array_element_10 (Math|Transform|MakeTransform "0, 0,-999999.000000" "0, 0, 0" "1,1,1") "Undefined" 0 0))
    (Rendering|SetActorHiddenInGame _returnvalue_10 true)
    (Collision|SetActorEnableCollision _returnvalue_10 false)
    (Utilities|Array|Add (Variables|ObstacleTiles|GetObstacleTilesDiff_4_Ref) _returnvalue_10))
  (Utilities|FlowControl|Sequence
    (:then_0
      (bind _returnvalue_11 (Game|SpawnActorfromClass "/Game/Blueprints/levelGenerator/BP_TileEnvi_Special_MegaCanion.BP_TileEnvi_Special_MegaCanion_C" (Math|Transform|MakeTransform "0, 0,-999999.000000" "0, 0, 0" "1,1,1") "Undefined" 0 0 0))
      (Rendering|SetActorHiddenInGame _returnvalue_11 true)
      (Collision|SetActorEnableCollision _returnvalue_11 false)
      (Variables|Default|SetCANION _returnvalue_11))
    (:then_1
      (Variables|Scores|SetY_LocationToAddScore (.y (Transformation|GetWorldLocation (Variables|/Game/Blueprints/Boat/BP_Pawn_VRBoat.BP_Pawn_VRBoat_C|GetDefaultSceneRoot (Variables|Default|GetPawn)))))
      (Utilities|FlowControl|Delay 0.2)
      (CallFunction|InitializeTilePlane)
      (CallFunction|InitializeTilePlane)
      (Variables|Default|SetTilesToSpecial (Math|Random|RandomIntegerinRange 4 6))
      (CallFunction|AddArch)
      (bind _returnvalue_12 (Utilities|Time|SetTimerbyFunctionName 0 "CheckStartTimer" 1.0 true))
      (Variables|Default|SetLishniyTaimer _returnvalue_12))))

(event EventTick
  (params (DeltaSeconds :type Float%20%28single-precision%29))
  ;[1 1 1] Tick
  (if (>= (.y (Transformation|GetWorldLocation (Variables|/Game/Blueprints/Boat/BP_Pawn_VRBoat.BP_Pawn_VRBoat_C|GetDefaultSceneRoot (Variables|Default|GetPawn)))) (+ (Variables|Scores|GetY_LocationToAddScore) (Variables|Scores|GetDistanceToGetPoint)))
    (bind _output_get (Variables|Scores|SetTotalScores (+ (Variables|Scores|GetTotalScores) (Variables|Scores|GetScoreMultiply))))
    (Variables|Scores|SetY_LocationToAddScore (.y (Transformation|GetWorldLocation (Variables|/Game/Blueprints/Boat/BP_Pawn_VRBoat.BP_Pawn_VRBoat_C|GetDefaultSceneRoot (Variables|Default|GetPawn)))))
    (Default|UpdateCounter (Variables|Default|GetPawn) _output_get)))

(fn ConstructionScript)

(fn AddTilePlane
  (Math|Integer|IncrementInt (Variables|Default|GetCallFunctionAddTile)
    (:%20%20
      (if (<= (Variables|Default|GetCallFunctionAddTile) (Variables|Default|GetTilesTo3ndDiff))
        (CallFunction|Add2ndDiffTiles)
        (elif (<= (Utilities|Time|GetGameTimeinSeconds) (Variables|Default|GetTimeEnd3dDiff))
          (CallFunction|Add3rdDiffTiles)
          (elif (not (Variables|Default|GetIs5thDiff))
            (CallFunction|Add4thDiffTiles)
            (else
              (CallFunction|Add5thDiffTiles))))))))

(fn SelectRandomTile
  (bind _tileswithenviromnent_ref_nowused (Variables|EnviromentTiles|GetTilesWithEnviromnent_Ref_NowUsed))
  (bind _tileswithenviromnent_ref (Variables|EnviromentTiles|GetTilesWithEnviromnent_Ref))
  (bind _output (Utilities|Array|Get(acopy) _tileswithenviromnent_ref_nowused))
  (LocalVariables|SetL_CurrentTile (Utilities|Array|Get(acopy) _tileswithenviromnent_ref (Math|Random|RandomIntegerinRange 0 (Utilities|Array|LastIndex _tileswithenviromnent_ref))))
  (Utilities|Array|AddUnique (Variables|EnviromentTiles|GetTilesWithEnviromnent_Ref_NowUsed) (LocalVariables|GetL_CurrentTile))
  (Utilities|Array|RemoveItem (Variables|EnviromentTiles|GetTilesWithEnviromnent_Ref) (LocalVariables|GetL_CurrentTile))
  (if (<= (Utilities|Array|Length (Variables|EnviromentTiles|GetTilesWithEnviromnent_Ref_NowUsed)) 6)
    (return (LocalVariables|GetL_CurrentTile))
    (else
      (Utilities|Array|AddUnique (Variables|EnviromentTiles|GetTilesWithEnviromnent_Ref) _output)
      (Utilities|Array|RemoveItem (Variables|EnviromentTiles|GetTilesWithEnviromnent_Ref_NowUsed) _output)
      (return (LocalVariables|GetL_CurrentTile)))))

(fn SelectObstacleTiles
  (params (Diff :type Integer) (TileType :type BP%20Tile%20Envi%20Object%20Reference))
  (bind _output_get (Variables|Diff|SetCurrentDiff Diff))
  (switch Utilities|FlowControl|Switch|SwitchonTypeOfEnvironment (Variables|/Game/Blueprints/levelGenerator/BP_TileEnvi.BP_TileEnvi_C|GetTileType TileType)
    (:NewEnumerator0
      (LocalVariables|SetL_Diff _output_get))
    (:NewEnumerator1
      (LocalVariables|SetL_Diff 5))
    (:NewEnumerator2
      (LocalVariables|SetL_Diff 6)))
  (LocalVariables|SetObstalceTile_ToSelect (Utilities|Select :Index (LocalVariables|GetL_Diff) :Option%200 (Variables|ObstacleTiles|GetObstacleTilesDiff_0_Ref) :Option%201 (Variables|ObstacleTiles|GetObstacleTilesDiff_1_Ref) :Option%202 (Variables|ObstacleTiles|GetObstacleTilesDiff_2_Ref) :Option%203 (Variables|ObstacleTiles|GetObstacleTilesDiff_3_Ref) :Option%204 (Variables|ObstacleTiles|GetObstacleTilesDiff_4_Ref) :Option%205 0 :Option%206 0))
  (for _array_element (Variables|ObstacleTiles|GetObstacleTiles_NowUsed)
    (Utilities|Array|RemoveItem (LocalVariables|GetObstalceTile_ToSelect) _array_element))
  (for _index (range 1 (Class|SceneComponent|GetNumChildrenComponents (Variables|/Game/Blueprints/levelGenerator/BP_TileEnvi.BP_TileEnvi_C|GetPointsSpawnObstacles TileType)))
    (bind _output_get_2 (LocalVariables|Settile (Utilities|Array|Get(acopy) (LocalVariables|GetObstalceTile_ToSelect) (Math|Random|RandomIntegerinRange 0 (Utilities|Array|LastIndex (LocalVariables|GetObstalceTile_ToSelect))))))
    (Utilities|Array|RemoveItem (LocalVariables|GetObstalceTile_ToSelect) _output_get_2)
    (Utilities|Array|Add (LocalVariables|Getsend) (LocalVariables|Gettile))
    (Utilities|Array|Add (Variables|ObstacleTiles|GetObstacleTiles_NowUsed) (LocalVariables|Gettile)))
  (return (LocalVariables|Getsend)))

(fn InitializeTilePlane
  (params (DIff :type Integer))
  (Math|Integer|IncrementInt (Variables|Default|GetCallFunctionAddTile)
    (:%20%20
      (bind _currenttile (CallFunction|SelectRandomTile))
      (bind _obstacletilestoteleport (CallFunction|SelectObstacleTiles DIff _currenttile))
      (bind _endpoint (Default|Initialize _currenttile _obstacletilestoteleport (Variables|Default|GetSpawnTLocation) (Variables|EnviromentTiles|GetCurentEnviTile)))
      (Variables|Default|SetSpawnTLocation _endpoint)
      (Variables|EnviromentTiles|SetCurentEnviTile _currenttile))))

(fn AddArch)

(fn SelectSpecialTile
  (bind _tileswithenviromnent_special_ref (Variables|EnviromentTiles|GetTilesWithEnviromnent_Special_Ref))
  (Utilities|IsValid (Variables|Default|GetNowUsedSpecialTile)
    (:Is%20Valid
      (Utilities|Array|Add (Variables|EnviromentTiles|GetTilesWithEnviromnent_Special_Ref) (Variables|Default|GetNowUsedSpecialTile)))
    (:Is%20Not%20Valid
      _))
  (bind _output_get (Variables|Default|SetNowUsedSpecialTile (Utilities|Array|Get(acopy) _tileswithenviromnent_special_ref (Math|Random|RandomIntegerinRange 0 (Utilities|Array|LastIndex _tileswithenviromnent_special_ref)))))
  (Utilities|Array|RemoveItem (Variables|EnviromentTiles|GetTilesWithEnviromnent_Special_Ref) _output_get)
  (return _output_get))

(fn Add2ndDiffTiles
  (bind _currenttile (CallFunction|SelectRandomTile))
  (bind _obstacletilestoteleport (CallFunction|SelectObstacleTiles 1 _currenttile))
  (bind _endpoint (Default|Teleport _currenttile _obstacletilestoteleport (Variables|EnviromentTiles|GetCurentEnviTile) (Variables|Default|GetSpawnTLocation)))
  (Variables|Default|SetSpawnTLocation _endpoint)
  (Variables|EnviromentTiles|SetCurentEnviTile _currenttile))

(fn Add3rdDiffTiles
  (if (== (Math|Integer|%(Integer) (Variables|Default|GetCallFunctionAddTile) (Variables|Default|GetTilesToSpecial)) 0)
    (bind _currenttile (CallFunction|SelectSpecialTile))
    (LocalVariables|SetL_CurrentSelectedTile _currenttile)
    (else
      (bind _currenttile_2 (CallFunction|SelectRandomTile))
      (LocalVariables|SetL_CurrentSelectedTile _currenttile_2)))
  (bind _obstacletilestoteleport (CallFunction|SelectObstacleTiles 2 (LocalVariables|GetL_CurrentSelectedTile)))
  (bind _endpoint (Default|Teleport (LocalVariables|GetL_CurrentSelectedTile) _obstacletilestoteleport (Variables|EnviromentTiles|GetCurentEnviTile) (Variables|Default|GetSpawnTLocation)))
  (Variables|Default|SetSpawnTLocation _endpoint)
  (Variables|EnviromentTiles|SetCurentEnviTile (LocalVariables|GetL_CurrentSelectedTile))
  (if (== (Math|Integer|%(Integer) (Variables|Scores|GetTotalPassedTiles) (Variables|EnviromentTiles|GetTilesToGate)) 0)
    (Default|Activate (Utilities|Array|Get(acopy) (Variables|Default|GetArches)) (Math|Vector|MakeVector 0.0 (+ (.y (Variables|Default|GetSpawnTLocation)) 6e+04) 0.0))))

(fn Add4thDiffTiles
  (if (Variables|Default|GetIs1stCall)
    (Default|StartHardLvL (Variables|Default|GetPawn))
    (Variables|Default|SetIs1stCall false))
  (if (>= (Variables|Default|Get4thDiffCallsCount) 9)
    (LocalVariables|SetL_CurrentSelectedTile (Variables|Default|GetCANION))
    (Variables|Default|SetIs5thDiff true)
    (else
      (Math|Integer|IncrementInt (Variables|Default|Get4thDiffCallsCount)
        (:%20%20
          (bind _currenttile (CallFunction|SelectRandomTile))
          (LocalVariables|SetL_CurrentSelectedTile _currenttile)))))
  (bind _obstacletilestoteleport (CallFunction|SelectObstacleTiles 3 (LocalVariables|GetL_CurrentSelectedTile)))
  (bind _endpoint (Default|Teleport (LocalVariables|GetL_CurrentSelectedTile) _obstacletilestoteleport (Variables|EnviromentTiles|GetCurentEnviTile) (Variables|Default|GetSpawnTLocation)))
  (Variables|Default|SetSpawnTLocation _endpoint)
  (Variables|EnviromentTiles|SetCurentEnviTile (LocalVariables|GetL_CurrentSelectedTile))
  (if (== (Math|Integer|%(Integer) (Variables|Scores|GetTotalPassedTiles) (Variables|EnviromentTiles|GetTilesToGate)) 0)
    (Default|Activate (Utilities|Array|Get(acopy) (Variables|Default|GetArches)) (Math|Vector|MakeVector 0.0 (+ (.y (Variables|Default|GetSpawnTLocation)) 6e+04) 0.0))))

(fn Add5thDiffTiles
  (if (== (Math|Integer|%(Integer) (Variables|Default|GetCallFunctionAddTile) (Variables|Default|GetTilesToSpecial)) 0)
    (bind _currenttile (CallFunction|SelectSpecialTile))
    (LocalVariables|SetL_CurrentSelectedTile _currenttile)
    (else
      (bind _currenttile_2 (CallFunction|SelectRandomTile))
      (LocalVariables|SetL_CurrentSelectedTile _currenttile_2)))
  (bind _obstacletilestoteleport (CallFunction|SelectObstacleTiles 4 (LocalVariables|GetL_CurrentSelectedTile)))
  (bind _endpoint (Default|Teleport (LocalVariables|GetL_CurrentSelectedTile) _obstacletilestoteleport (Variables|EnviromentTiles|GetCurentEnviTile) (Variables|Default|GetSpawnTLocation)))
  (Variables|Default|SetSpawnTLocation _endpoint)
  (Variables|EnviromentTiles|SetCurentEnviTile (LocalVariables|GetL_CurrentSelectedTile))
  (if (== (Math|Integer|%(Integer) (Variables|Scores|GetTotalPassedTiles) (Variables|EnviromentTiles|GetTilesToGate)) 0)
    (Default|Activate (Utilities|Array|Get(acopy) (Variables|Default|GetArches)) (Math|Vector|MakeVector 0.0 (+ (.y (Variables|Default|GetSpawnTLocation)) 6e+04) 0.0))))

(fn CheckStartTimer
  (if (>= (Variables|Scores|GetTotalPassedTiles) 5)
    (Default|StartNormalLvl (Variables|Default|GetPawn) (Variables|Default|GetSecondsTo4thDiff))
    (CallFunction|StartTimer)
    (Utilities|Time|ClearandInvalidateTimerbyHandle (Variables|Default|GetLishniyTaimer))))