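; Reusable environment tile for the auto-generated boat level, placed with pooled obstacle actors snapped to its spawn points.
; Teleport shows the tile, swings it up via Tick-driven roll and returns its end point, while Initialize places it without animation.
; The boat overlapping TileEnd updates GameMode counters, requests another tile and wakes the previous tile.
; That tile rotates down, then parks itself and its obstacles hidden far away instead of destroying them.
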(event OnComponentBeginOverlap(TileEnd)
  (params (OverlappedComponent :type Primitive%20Component%20Object%20Reference) (OtherActor :type Actor%20Object%20Reference) (OtherComp :type Primitive%20Component%20Object%20Reference) (OtherBodyIndex :type Integer) (bFromSweep :type Boolean) (SweepResult :type Hit%20Result%20Structure%20%28by%20ref%29))
  (bind _gamemode (Variables|Default|GetGameMode))
  (Utilities|Casting|CastToBP_Pawn_VRBoat OtherActor
    (:then
      _)
    (:CastFailed
      (Utilities|Casting|CastToBoatKeyboard OtherActor)))
  (Collision|SetCollisionEnabled (Variables|Default|GetTileEnd) "NoCollision")
  (Math|Integer|IncrementInt (Variables|/Game/Blueprints/levelGenerator/AutoLVL_GameMode.AutoLVL_GameMode_C|GetPassedTiles _gamemode)
    (:%20%20
      (Math|Integer|IncrementInt (Variables|/Game/Blueprints/levelGenerator/AutoLVL_GameMode.AutoLVL_GameMode_C|GetTotalPassedTiles _gamemode)
        (:%20%20
          (Default|AddTilePlane _gamemode)
          (Variables|Default|SetAlphaRot 0.0)
          (Variables|Default|SetUp/Down-True/fals false)
          (CallFunction|OnEnd))))))

(event Custom|RotateUp)

(event Custom|RotateDown)

(event EventBeginPlay
  (bind _asauto_lvl_game_mode (Utilities|Casting|CastToAutoLVL_GameMode (Game|GetGameMode)))
  (Variables|Default|SetGameMode _asauto_lvl_game_mode)
  ;[1 1 1] Comment
  (bind _asbp_pawn_vrboat (Utilities|Casting|CastToBP_Pawn_VRBoat (Game|Player|GetPlayerPawn 0)))
  (Variables|Default|SetPawn _asbp_pawn_vrboat))

(event EventTick
  (params (DeltaSeconds :type Float%20%28single-precision%29))
  (bind _returnvalue (Transformation|GetActorLocation))
  (if (Variables|Default|GetUp/Down-True/fals)
    (bind _output_get (Variables|Default|SetAlphaRot (Math|Float|Clamp(Float) (+ (Variables|Default|GetAlphaRot) (* (Utilities|Time|GetWorldDeltaSeconds) (Variables|Default|GetSpeedRotator_Div))))))
    (if (<= _output_get 0.99)
      (Transformation|SetRelativeRotation (Variables|Default|GetTileRotatePointUp) (Math|Rotator|MakeRotator (Math|Float|Lerp 6e+01 0.0 (Variables|Default|GetAlphaRot)) 0.0 0.0) false false)
      (else
        (Variables|Default|SetAlphaRot 0.0)
        (Transformation|SetRelativeRotation (Variables|Default|GetTileRotatePointUp) (Math|Rotator|MakeRotator 0.0 0.0 0.0) false false)
        (Transformation|SetActorLocation (Math|Vector|MakeVector (.x _returnvalue) (.y _returnvalue) 0.0) false false)
        (Collision|SetActorEnableCollision true)
        (Actor|Tick|SetActorTickEnabled false)))
    (else
      (bind _output_get_2 (Variables|Default|SetAlphaRot (Math|Float|Clamp(Float) (+ (Variables|Default|GetAlphaRot) (* (Utilities|Time|GetWorldDeltaSeconds) (Variables|Default|GetSpeedRotator_Div))))))
      (if (<= _output_get_2 0.99)
        (Transformation|SetRelativeRotation (Variables|Default|GetTileRotatePointDown) (Math|Rotator|MakeRotator (Math|Float|Lerp 0.0 -3e+01 (Variables|Default|GetAlphaRot)) 0.0 0.0) false false)
        (else
          (CallFunction|RemoveSelf))))))

(fn ConstructionScript)

(fn AddObstacleTiles
  (params (obstacleTiles :type Array%20of%20Obstacle%20Tile%20Main%20Object%20References))
  (for (_array_element _array_index) obstacleTiles
    (Rendering|SetActorHiddenInGame _array_element false)
    (Collision|SetActorEnableCollision _array_element true)
    (Transformation|AttachComponentToComponent _array_element (.Item (CallFunction|GetPointsLocation _array_index)) "None" "SnapToTarget" "SnapToTarget" "SnapToTarget" true)
    (Utilities|Array|AddUnique (Variables|Default|GetObstacleTiles) _array_element)))

(fn GetPointsLocation
  (params (Index :type Integer))
  (bind _pointsspawnobstacles (Variables|Default|GetPointsSpawnObstacles))
  (bind _children (Components|GetChildrenComponents _pointsspawnobstacles false))
  (bind _output (Utilities|Array|Get(acopy) _children Index))
  (return (Transformation|GetWorldLocation _output) _output))

(fn RemoveObstacleTiles
  (for _array_element (Variables|Default|GetObstacleTiles)
    (Utilities|Array|RemoveItem (Variables|/Game/Blueprints/levelGenerator/AutoLVL_GameMode.AutoLVL_GameMode_C|GetObstacleTiles_NowUsed (Variables|Default|GetGameMode)) _array_element))
  (for _array_element_2 (Variables|Default|GetObstacleTiles)
    (Transformation|DetachFromActor _array_element_2 "KeepWorld" "KeepWorld" "KeepWorld")
    (Transformation|Teleport _array_element_2 "-50000.000000, 0,-999999.000000" "0, 0, 0")
    (Rendering|SetActorHiddenInGame _array_element_2 true)
    (Collision|SetActorEnableCollision _array_element_2 false))
  (Utilities|Array|Clear (Variables|Default|GetObstacleTiles)))

(fn RemoveSelf
  (Variables|Default|SetAlphaRot 0.0)
  (Actor|Tick|SetActorTickEnabled false)
  (Transformation|SetRelativeRotation (Variables|Default|GetTileRotatePointDown) "0, 0, 0" false false)
  (Transformation|Teleport "-50000.000000, 0,-999999.000000" "0, 0, 0")
  (Rendering|SetActorHiddenInGame true)
  (Collision|SetActorEnableCollision false)
  (CallFunction|RemoveObstacleTiles))

(fn Teleport
  (params (obstacleTiles :type Array%20of%20Obstacle%20Tile%20Main%20Object%20References) (PrevTile :type BP%20Tile%20Envi%20Object%20Reference) (Location :type Vector))
  (Variables|Default|SetPrevTile PrevTile)
  (Transformation|Teleport (Math|Vector|MakeVector (.x Location) (.y Location) 0.0) "0, 0,0.000000")
  (CallFunction|AddObstacleTiles obstacleTiles)
  (Rendering|SetActorHiddenInGame false)
  (Collision|SetActorEnableCollision true)
  (Variables|Default|SetUp/Down-True/fals true)
  (Transformation|SetRelativeRotation (Variables|Default|GetTileRotatePointUp) (Math|Rotator|MakeRotator 6e+01 0.0 0.0) false false)
  (Actor|Tick|SetActorTickEnabled true)
  (return (Transformation|GetWorldLocation (Variables|Default|GetEndPoint))))

(fn Initialize
  (params (obstacleTiles :type Array%20of%20Obstacle%20Tile%20Main%20Object%20References) (Location :type Vector) (PrevTile :type BP%20Tile%20Envi%20Object%20Reference))
  (Variables|Default|SetPrevTile PrevTile)
  (Transformation|Teleport (Math|Vector|MakeVector (.x Location) (.y Location) 0.0) "0, 0,0.000000")
  (CallFunction|AddObstacleTiles obstacleTiles)
  (Rendering|SetActorHiddenInGame false)
  (Collision|SetActorEnableCollision true)
  (return (Transformation|GetWorldLocation (Variables|Default|GetEndPoint))))

(fn OnEnd
  (bind _prevtile (Variables|Default|GetPrevTile))
  (Utilities|IsValid _prevtile
    (:Is%20Valid
      (Actor|Tick|SetActorTickEnabled _prevtile true)
      (Collision|SetCollisionEnabled (Variables|BP_TileEnvi_C|GetTileEnd _prevtile) "QueryOnly"))))