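; BP_TileEnvi_Special is a level-generator tile that temporarily changes the VR boat's environment sounds, gain and speed coefficient.
; When the boat overlaps SpecialTileStart, Start applies the tile's values through the Pawn reference, and overlapping TileEnd resets them.
; Start disables the start trigger's collision, and a five-second delay marked as a workaround ("Kostyel") re-enables it as query-only.
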(event OnComponentBeginOverlap(SpecialTileStart)
  (params (OverlappedComponent :type Primitive%20Component%20Object%20Reference) (OtherActor :type Actor%20Object%20Reference) (OtherComp :type Primitive%20Component%20Object%20Reference) (OtherBodyIndex :type Integer) (bFromSweep :type Boolean) (SweepResult :type Hit%20Result%20Structure%20%28by%20ref%29))
  (Utilities|Casting|CastToBP_Pawn_VRBoat OtherActor)
  (CallFunction|Start)
  ;[1 1 1] Kostyel
  (Utilities|FlowControl|Delay 5.0)
  (Collision|SetCollisionEnabled (Variables|Default|GetSpecialTileStart) "QueryOnly"))

(event OnComponentBeginOverlap(TileEnd)
  (params (OverlappedComponent :type Primitive%20Component%20Object%20Reference) (OtherActor :type Actor%20Object%20Reference) (OtherComp :type Primitive%20Component%20Object%20Reference) (OtherBodyIndex :type Integer) (bFromSweep :type Boolean) (SweepResult :type Hit%20Result%20Structure%20%28by%20ref%29))
  (Utilities|Casting|CastToBP_Pawn_VRBoat OtherActor)
  (CallFunction|End))

(event EventBeginPlay
  (|CallParentFunction))

(event Collision|EventActorBeginOverlap
  (params (OtherActor :type Actor%20Object%20Reference)))

(event EventTick
  (params (DeltaSeconds :type Float%20%28single-precision%29))
  (|CallParentFunction DeltaSeconds))

(fn ConstructionScript
  (|CallParentFunction))

(fn Start
  (bind _pawn (Variables|Default|GetPawn))
  (Collision|SetCollisionEnabled (Variables|Default|GetSpecialTileStart) "NoCollision")
  (Default|ChangeTypeOfEnviroment (Variables|/Game/Blueprints/Boat/BP_Pawn_VRBoat.BP_Pawn_VRBoat_C|GetSounds (Variables|Default|GetPawn)) (Variables|Default|GetTileType))
  (Default|Gain _pawn (Variables|Default|GetGain))
  (Default|SetSpeedKoef _pawn (Variables|Default|GetSpeedKoef)))

(fn End
  (bind _pawn (Variables|Default|GetPawn))
  (Default|ChangeTypeOfEnviroment (Variables|/Game/Blueprints/Boat/BP_Pawn_VRBoat.BP_Pawn_VRBoat_C|GetSounds (Variables|Default|GetPawn)) "NewEnumerator0")
  (Default|SetSpeedKoef _pawn 1.0)
  (Default|Gain _pawn 1.0))