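; A Blueprint pawn or character that provides non-VR mouse look and manual rotation of a component named Left.
; MouseX and MouseY axes feed controller yaw and pitch input, with pitch inverted.
; The NoVrControl axis adds relative yaw to Left, and NoVRSensetivity adds scaled relative roll to it.
; BeginPlay, overlap and Tick are empty, and the Right component is unused.
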(event EventBeginPlay)

(event Collision|EventActorBeginOverlap
  (params (OtherActor :type Actor%20Object%20Reference)))

(event EventTick
  (params (DeltaSeconds :type Float%20%28single-precision%29)))

(event Input|AxisEvents|InputAxisNoVrControl
  (params (AxisValue :type Float%20%28single-precision%29))
  (Transformation|AddRelativeRotation (Variables|Default|Getleft) (Math|Rotator|MakeRotator 0.0 0.0 AxisValue) false false))

(event Input|AxisEvents|InputAxisNoVRSensetivity
  (params (AxisValue :type Float%20%28single-precision%29))
  (Transformation|AddRelativeRotation (Variables|Default|Getleft) (Math|Rotator|MakeRotator (* AxisValue 5.0) 0.0 0.0) false false))

(event Input|MouseEvents|MouseX
  (params (AxisValue :type Float%20%28single-precision%29))
  (Pawn|Input|AddControllerYawInput AxisValue))

(event Input|MouseEvents|MouseY
  (params (AxisValue :type Float%20%28single-precision%29))
  (Pawn|Input|AddControllerPitchInput (* AxisValue -1.0)))

(fn ConstructionScript)