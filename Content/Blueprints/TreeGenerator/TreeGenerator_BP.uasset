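; TreeGenerator_BP is a tree generator actor that assembles a tree from a stem mesh and a crown mesh.
; Its construction script sets the stem from the SteamType selection and gathers the crown shapes enabled by boolean flags into an array.
; It assigns a random crown from that array on each construction run.
; Nodes for setting the scene's rotation and scale exist but are not connected.
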(fn ConstructionScript
  (bind _tree (Variables|Default|GetTree))
  (if (Variables|Default|GetSphere)
    (Utilities|Array|AppendArray (Variables|Default|GetTMP) (Variables|Default|GetCrownSphere)))
  (if (Variables|Default|GetTriangle)
    (Utilities|Array|AppendArray (Variables|Default|GetTMP) (Variables|Default|GetCrownTriangle)))
  (if (Variables|Default|GetSquare)
    (Utilities|Array|AppendArray (Variables|Default|GetTMP) (Variables|Default|GetCrownSquare)))
  (if (Variables|Default|GetHoleSquare)
    (Utilities|Array|AppendArray (Variables|Default|GetTMP) (Variables|Default|GetCrownHoleSquare)))
  (if (Variables|Default|GetThor)
    (Utilities|Array|AppendArray (Variables|Default|GetTMP) (Variables|Default|GetCrownThor)))
  (switch Utilities|FlowControl|Switch|SwitchonTreeSteamHeigst (Variables|Default|GetSteamType)
    (:NewEnumerator0
      (Components|StaticMesh|SetStaticMesh _tree "/Game/Geometry/Tree/Stem/Stem_01.Stem_01"))
    (:NewEnumerator1
      (Components|StaticMesh|SetStaticMesh _tree "/Game/Geometry/Tree/Stem/Stem_02.Stem_02"))
    (:NewEnumerator2
      (Components|StaticMesh|SetStaticMesh _tree "/Game/Geometry/Tree/Stem/Stem_03.Stem_03"))
    (:NewEnumerator3
      (Components|StaticMesh|SetStaticMesh _tree "/Game/Geometry/Tree/Stem/Stem_04.Stem_04")))
  (Components|StaticMesh|SetStaticMesh (Variables|Default|GetTreeHead) (Utilities|Array|Get(acopy) (Variables|Default|GetTMP) (Math|Random|RandomIntegerinRange 0 (Utilities|Array|LastIndex (Variables|Default|GetTMP))))))