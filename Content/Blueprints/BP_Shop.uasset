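; BP_Shop is the booster shop, selling three boosters (magnet, ray and double collectible) for saved collectibles.
; It caches the AutoLVL_GameMode on BeginPlay and uses its Load and Save as the wallet.
; Each buy event checks the balance covers the fixed price, saves the deduction and calls that booster's CallBuyBooster hook.
; Success and insufficient-funds results are only printed as debug strings.
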(event Custom|Buy1Booster
  (bind _gamemode (Variables|Default|GetGameMode))
  (bind _smallcolls (Default|Load _gamemode))
  (if (> _smallcolls 4)
    (Development|PrintString "Magneet" true true "(R=0.000000,G=0.660000,B=1.000000,A=1.000000)" 1e+01)
    (Default|Save _gamemode _smallcolls -5)
    (Default|CallBuyBooster1)
    (else
      (Development|PrintString "nehvataetNaMagneet" true true "(R=0.000000,G=0.660000,B=1.000000,A=1.000000)" 1e+01))))

(event Custom|Buy3Booster
  (bind _gamemode (Variables|Default|GetGameMode))
  (bind _smallcolls (Default|Load _gamemode))
  (if (> _smallcolls 4)
    (Development|PrintString "DoubleCol" true true "(R=0.000000,G=0.660000,B=1.000000,A=1.000000)" 1e+01)
    (Default|Save _gamemode _smallcolls -5)
    (Default|CallBuyBooster3)
    (else
      (Development|PrintString "nehvataetNaDoubleCol" true true "(R=0.000000,G=0.660000,B=1.000000,A=1.000000)" 1e+01))))

(event Custom|Buy2Booster
  (bind _gamemode (Variables|Default|GetGameMode))
  (bind _smallcolls (Default|Load _gamemode))
  (if (> _smallcolls 4)
    (Development|PrintString "Ray" true true "(R=0.000000,G=0.660000,B=1.000000,A=1.000000)" 1e+01)
    (Default|Save _gamemode _smallcolls -5)
    (Default|CallBuyBooster2)
    (else
      (Development|PrintString "nehvataetNaRay" true true "(R=0.000000,G=0.660000,B=1.000000,A=1.000000)" 1e+01))))

(event EventBeginPlay
  (bind _asauto_lvl_game_mode (Utilities|Casting|CastToAutoLVL_GameMode (Game|GetGameMode)))
  (Variables|Default|SetGameMode _asauto_lvl_game_mode))

(fn ConstructionScript)