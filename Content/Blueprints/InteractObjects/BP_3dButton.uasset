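; BP_3dButton is a 3D button actor that serves as a yes or close choice for its parent BP_InteractObject.
; On BeginPlay it caches that parent actor, and Act calls the parent's Yes or Close based on IsYes, then ToggleActive.
; The construction script applies ButtonMaterial to the mesh, while helper events set actor scale and collider box position.
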(event Custom|SetScale
  (params (Scale :type Vector))
  (Transformation|SetActorScale3D Scale))

(event Custom|SetColliderOffset
  (params (DeltaLocation :type Vector))
  (Transformation|SetRelativeLocation (Variables|Default|GetBox) DeltaLocation false false))

(event EventBeginPlay
  (bind _asbp_interact_object (Utilities|Casting|CastToBP_InteractObject (Actor|GetParentActor)))
  (Variables|Default|SetParent _asbp_interact_object))

(event EventAct
  (bind _parent (Variables|Default|GetParent))
  (if (Variables|Default|GetIsYes)
    (Default|Yes _parent)
    (else
      (Default|Close _parent)))
  (Default|ToggleActive _parent))

(fn ConstructionScript
  (Rendering|Material|SetMaterial (Variables|Character|GetMesh) 0 (Variables|Default|GetButtonMaterial))
  (|CallParentFunction))