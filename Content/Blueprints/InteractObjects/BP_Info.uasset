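; BP_Info is an interactable object that shows and hides an info pop-up with a 3D close button.
; On BeginPlay it caches the BP_3dButton from the ButtonClose child actor.
; Act calls its parent, plays a sound and runs the ShowHideInfo timeline, which scales the pop-up and button together.
; Close calls its parent and reverses that timeline, and End fires whenever the timeline finishes.
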(event EventBeginPlay
  (bind _asbp_3d_button (Utilities|Casting|CastToBP_3dButton (Variables|/Script/Engine.ChildActorComponent|GetChildActor (Variables|Default|GetButtonClose))))
  (Variables|Default|SetButton _asbp_3d_button))

(event EventAct
  (|CallParentFunction)
  (Audio|PlaySound2D "/Game/Sounds/UI_Sounds/Pop_Up.Pop_Up")
  (bind (_direction _scale) (Timeline|Show/Hide%20Info PlayFromStart)
    (:Update
      (Transformation|SetWorldScale3D (Variables|Default|GetPopUp) (Math|Vector|MakeVector _scale _scale _scale))
      (Default|SetScale (Variables|Default|GetButton) (Math|Vector|MakeVector _scale _scale _scale)))
    (:Finished
      (CallFunction|End))))

(event EventClose
  (|CallParentFunction)
  (bind (_direction _scale) (Timeline|Show/Hide%20Info ReverseFromEnd)
    (:Update
      (Transformation|SetWorldScale3D (Variables|Default|GetPopUp) (Math|Vector|MakeVector _scale _scale _scale))
      (Default|SetScale (Variables|Default|GetButton) (Math|Vector|MakeVector _scale _scale _scale)))
    (:Finished
      (CallFunction|End))))

(fn ConstructionScript
  (|CallParentFunction))