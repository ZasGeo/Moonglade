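; BP_SwitchGamemode is an interactable object that toggles the game mode's IsSimpleGame flag.
; On BeginPlay it highlights or lowlights itself to match the current flag.
; Act flips the flag without calling the parent Act, updates the highlight and prints the new value in a state-specific color.
; ToggleActive is overridden as a no-op, and Restart re-enables actor collision.
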(event EventAct
  (bind _gamemode (Variables|Default|GetGamemode))
  (bind _output_get (Variables|/Game/Blueprints/levelGenerator/AutoLVL_GameMode.AutoLVL_GameMode_C|SetIsSimpleGame _gamemode (not (Variables|/Game/Blueprints/levelGenerator/AutoLVL_GameMode.AutoLVL_GameMode_C|GetIsSimpleGame _gamemode))))
  (if _output_get
    (CallFunction|Highlight)
    (Development|PrintString (Utilities|String|ToString(Boolean) _output_get) true true "(R=1.000000,G=0.000000,B=0.712466,A=1.000000)" 1e+01)
    (else
      (CallFunction|Lowlight)
      (Development|PrintString (Utilities|String|ToString(Boolean) _output_get) true true "(R=0.293339,G=1.000000,B=0.000000,A=1.000000)" 1e+01))))

(event EventToggleActive)

(event EventRestart
  (Collision|SetActorEnableCollision true))

(event EventBeginPlay
  (|CallParentFunction)
  (if (Variables|/Game/Blueprints/levelGenerator/AutoLVL_GameMode.AutoLVL_GameMode_C|GetIsSimpleGame (Variables|Default|GetGamemode))
    (CallFunction|Highlight)
    (else
      (CallFunction|Lowlight))))

(fn ConstructionScript
  (|CallParentFunction))