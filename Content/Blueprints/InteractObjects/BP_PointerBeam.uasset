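; BP_PointerBeam is a pointer beam actor that draws a curved spline mesh between a Start and an End component.
; Each tick it moves End to WorldEnd, faces it toward Start, and rebuilds the curve with distance-scaled tangents, tilting the start tangent for an arc.
; BeamAct plays a timeline that drives the Time parameter of a dynamic material created in the construction script, and SwitchVisability toggles the mesh.
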(event Custom|SwitchVisability
  (Rendering|ToggleVisibility (Variables|Default|GetSplineMesh) false))

(event Custom|BeamAct
  (bind _newtrack_0 (Timeline|Beam PlayFromStart)
    (:Update
      (Rendering|Material|SetScalarParameterValue (Variables|Default|GetM_Beam) "Time" _newtrack_0 :!class /Script/Engine.MaterialInstanceDynamic))))

(event EventTick
  (params (DeltaSeconds :type Float%20%28single-precision%29))
  (bind _start (Variables|Default|GetStart))
  (bind _end (Variables|Default|GetEnd))
  (bind _end_2 (Variables|Default|GetEnd))
  (bind _returnvalue (Transformation|GetRelativeTransform _start))
  (bind _returnvalue_2 (Transformation|GetRelativeTransform _end))
  (bind (_location _rotation _scale) (Math|Transform|BreakTransform _returnvalue))
  (bind (_location_2 _rotation_2 _scale_2) (Math|Transform|BreakTransform _returnvalue_2))
  (bind _returnvalue_3 (- _location _location_2))
  (bind _returnvalue_4 (Math|Vector|VectorLength _returnvalue_3))
  (Transformation|SetWorldLocation (Variables|Default|GetEnd) (Variables|Default|GetWorldEnd) false false)
  (Transformation|SetWorldRotation _end_2 (Math|Rotator|FindLookatRotation (Transformation|GetWorldLocation _end_2) (Transformation|GetWorldLocation (Variables|Default|GetStart))) false false)
  (SplineMesh|SetStartandEnd (Variables|Default|GetSplineMesh) _location (* (* (Math|Vector|RotateVectorAroundAxis (Math|Vector|GetForwardVector _rotation) -2e+01 (Math|Vector|GetRightVector _rotation)) _scale) (* _returnvalue_4 (Variables|Default|GetStartKoef))) _location_2 (* (* (Math|Vector|GetForwardVector _rotation_2) _scale_2) (* _returnvalue_4 (Variables|Default|GetEndKoef))) true :!class /Script/Engine.SplineMeshComponent))

(fn ConstructionScript
  (bind _splinemesh (Variables|Default|GetSplineMesh))
  (bind _returnvalue (Rendering|Material|CreateDynamicMaterialInstance _splinemesh 0 (Rendering|Material|GetMaterial _splinemesh 0) :!class /Script/Engine.PrimitiveComponent))
  (Variables|Default|SetM_Beam _returnvalue))