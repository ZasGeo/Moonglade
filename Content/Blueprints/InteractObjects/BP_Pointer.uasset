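; BP_Pointer is one of a pair of hand pointers that highlight and trigger BP_InteractParent objects.
; A Cube overlap highlights the object, aims the Beam at it and disables the other hand's collision until the overlap ends.
; Action passes a gate to call Act on the overlapped object, then closes both hands' gates and toggles their collision profiles between buttons and objects.
; An end-of-action event is bound on the object, and Free reopens both gates.
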(event OnComponentBeginOverlap(Cube)
  (params (OverlappedComponent :type Primitive%20Component%20Object%20Reference) (OtherActor :type Actor%20Object%20Reference) (OtherComp :type Primitive%20Component%20Object%20Reference) (OtherBodyIndex :type Integer) (bFromSweep :type Boolean) (SweepResult :type Hit%20Result%20Structure%20%28by%20ref%29))
  (bind _asbp_interact_parent (Utilities|Casting|CastToBP_InteractParent OtherActor))
  (Collision|SetActorEnableCollision (Variables|Default|GetOtherHand) false)
  (Default|Highlight _asbp_interact_parent)
  (Variables|Default|SetDebugActor _asbp_interact_parent)
  (Effects|Components|ParticleSystem|SetActorParameter (Variables|Default|GetBeam) "BeamTarget" _asbp_interact_parent)
  (Audio|PlaySound2D "/Game/Sounds/UI_Sounds/Button_Point.Button_Point"))

(event OnComponentEndOverlap(Cube)
  (params (OverlappedComponent :type Primitive%20Component%20Object%20Reference) (OtherActor :type Actor%20Object%20Reference) (OtherComp :type Primitive%20Component%20Object%20Reference) (OtherBodyIndex :type Integer))
  (bind _asbp_interact_parent (Utilities|Casting|CastToBP_InteractParent OtherActor))
  (Default|Lowlight _asbp_interact_parent)
  (Variables|Default|SetDebugActor 0)
  (Effects|Components|ParticleSystem|SetActorParameter (Variables|Default|GetBeam) "BeamTarget" 0)
  (Collision|SetActorEnableCollision (Variables|Default|GetOtherHand) true))

(event Custom|Action
  (Utilities|FlowControl|Gate false
    (:Exit
      (bind _object (CallFunction|GetInteraction))
      (Utilities|IsValid _object
        (:Is%20Valid
          (Audio|PlaySound2D "/Game/Sounds/UI_Sounds/Button_Press.Button_Press")
          (EventDispatchers|BindEventtoEndOfAction _object (EventDispatchers|CreateEvent :!event Free))
          (Default|Act _object)
          (CallFunction|OnAct))))))

(event Custom|Open
  (Utilities|FlowControl|Gate false) ; enters at Open
)

(event Custom|Close
  (Utilities|FlowControl|Gate false) ; enters at Close
)

(event EventBeginPlay
  (Utilities|FlowControl|Delay 0.2)
  (bind _outactors (Actor|GetAllActorsOfClass "BP_Pointer_C"))
  (for _array_element _outactors
    (if (!= _array_element self)
      (Variables|Default|SetOtherHand _array_element))))

(event EventTick
  (params (DeltaSeconds :type Float%20%28single-precision%29))
  (Transformation|SetWorldRotation (Variables|Default|GetBeam) "0.0,0.0,0.0" false false))

(fn ConstructionScript)

(fn GetInteraction
  (bind _asbp_interact_parent (Utilities|Casting|CastToBP_InteractParent (Utilities|Array|Get(acopy) (Collision|GetOverlappingActors (Variables|Default|GetCube) "/Game/Blueprints/InteractObjects/BP_InteractParent.BP_InteractParent_C" :!class /Script/Engine.PrimitiveComponent)))
    (:then
      (return _asbp_interact_parent))
    (:CastFailed
      (return 0))))

(fn SetOverlapButtons
  (Collision|SetCollisionProfileName (Variables|Default|GetCube) "OverlapButton" :!class /Script/Engine.PrimitiveComponent)
  (Variables|Default|SetOverlapButt true))

(fn SetOverlapObject
  (Collision|SetCollisionProfileName (Variables|Default|GetCube) "OverlapObject" :!class /Script/Engine.PrimitiveComponent)
  (Variables|Default|SetOverlapButt false))

(fn SwitchOverlaps
  (if (Variables|Default|GetOverlapButt)
    (CallFunction|SetOverlapObject)
    (else
      (CallFunction|SetOverlapButtons))))

(fn OnAct
  (bind _otherhand (Variables|Default|GetOtherHand))
  (CallFunction|Close)
  (CallFunction|SwitchOverlaps)
  (CallFunction|Close _otherhand)
  (CallFunction|SwitchOverlaps _otherhand))

(fn Free
  (CallFunction|Open)
  (CallFunction|Open (Variables|Default|GetOtherHand)))

(fn SetCollison
  (params (Coll :type ECollisionEnabled%20Enum))
  (Development|PrintString (Utilities|String|Append (Utilities|GetDisplayName (Variables|Default|GetCube)) "    " (Utilities|Select :Index Coll :NoCollision "no" :QueryOnly "col" :PhysicsOnly "0" :QueryAndPhysics "0")))
  (Collision|SetCollisionEnabled (Variables|Default|GetCube) Coll))