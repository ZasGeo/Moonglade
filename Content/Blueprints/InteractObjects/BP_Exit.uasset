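; BP_Exit is an interactable object that shows an exit confirmation pop-up and quits the game.
; It extends a parent interactable: Act plays a sound and a timeline that scales up the pop-up and its two BP_3dButton child actors, then offsets their colliders.
; Close reverses the timeline, and Yes runs the "exit" console command.
; Collision-toggling nodes for the box and buttons are present but never run.
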(event EventAct
  (|CallParentFunction)
  (Audio|PlaySound2D "/Game/Sounds/UI_Sounds/Pop_Up.Pop_Up")
  (bind (_direction _scale) (Timeline|Show/Hide%20Buttons PlayFromStart)
    (:Update
      (Transformation|SetRelativeScale3D (Variables|Default|GetPopUp) (Math|Vector|MakeVector _scale _scale _scale))
      (Default|SetScale (Variables|Default|GetButtonClose_Child) (Math|Vector|MakeVector _scale _scale _scale)))
    (:Finished
      (CallFunction|End)
      (Default|SetColliderOffset (Variables|Default|GetButtonClose_Child) "0.000000,450.000000,0.000000")
      (Default|SetColliderOffset (Variables|Default|GetButtonYes_CHild) "0.000000,-450.000000,0.000000"))))

(event EventBeginPlay
  (bind _asbp_3d_button (Utilities|Casting|CastToBP_3dButton (Variables|/Script/Engine.ChildActorComponent|GetChildActor (Variables|Default|GetButtonClose))))
  (Variables|Default|SetButtonClose_Child _asbp_3d_button)
  (bind _asbp_3d_button_2 (Utilities|Casting|CastToBP_3dButton (Variables|/Script/Engine.ChildActorComponent|GetChildActor (Variables|Default|GetButtonYes))))
  (Variables|Default|SetButtonYes_CHild _asbp_3d_button_2))

(event EventClose
  (|CallParentFunction)
  (bind (_direction _scale) (Timeline|Show/Hide%20Buttons ReverseFromEnd)
    (:Update
      (Transformation|SetRelativeScale3D (Variables|Default|GetPopUp) (Math|Vector|MakeVector _scale _scale _scale))
      (Default|SetScale (Variables|Default|GetButtonClose_Child) (Math|Vector|MakeVector _scale _scale _scale)))
    (:Finished
      (CallFunction|End)
      (Default|SetColliderOffset (Variables|Default|GetButtonClose_Child) "0.000000,450.000000,0.000000")
      (Default|SetColliderOffset (Variables|Default|GetButtonYes_CHild) "0.000000,-450.000000,0.000000"))))

(event EventYes
  (Development|ExecuteConsoleCommand "exit"))

(fn ConstructionScript
  (|CallParentFunction))