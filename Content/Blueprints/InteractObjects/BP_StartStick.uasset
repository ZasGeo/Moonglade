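; BP_StartStick is an interact object that starts the game for the VR boat pawn.
; On BeginPlay it caches the pawn and levels PointToMove to the Start actor's height.
; Act disables its own and the Switch's collision, triggers sound, game mode and controller changes, then runs a timeline that ends by calling StartSail and End.
; Timeline-driven boat movement and pitch nodes exist but are never executed.
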(event EventAct
  (|CallParentFunction)
  (Collision|SetActorEnableCollision false)
  (Collision|SetActorEnableCollision (Variables|Default|GetSwitch) false)
  (Default|Arch (Variables|/Game/Blueprints/Boat/BP_Pawn_VRBoat.BP_Pawn_VRBoat_C|GetSounds (Variables|Default|GetPlayer)))
  (Default|Start (Variables|/Game/Blueprints/Boat/BP_Pawn_VRBoat.BP_Pawn_VRBoat_C|GetGameMode (Variables|Default|GetPlayer)))
  (Default|SetGameMode (Variables|/Game/Blueprints/Boat/BP_Pawn_VRBoat.BP_Pawn_VRBoat_C|GetLeftController (Variables|Default|GetPlayer)))
  (bind (_direction _alphapos _rot) (Timeline|Timeline_0 PlayFromStart)
    (:Finished
      (Default|StartSail (Variables|Default|GetPlayer))
      (CallFunction|End))))

(event EventBeginPlay
  (bind _pointtomove (Variables|Default|GetPointToMove))
  (bind _returnvalue (Transformation|GetWorldLocation _pointtomove))
  (bind _asbp_pawn_vrboat (Utilities|Casting|CastToBP_Pawn_VRBoat (Game|Player|GetPlayerPawn 0)))
  (Variables|Default|SetPlayer _asbp_pawn_vrboat)
  (Transformation|SetWorldLocation _pointtomove (Math|Vector|MakeVector (.x _returnvalue) (.y _returnvalue) (.z (Transformation|GetActorLocation (Variables|Default|GetStart)))) false false))

(fn ConstructionScript
  (|CallParentFunction))