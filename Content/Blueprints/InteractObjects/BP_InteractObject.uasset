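; BP_InteractObject is an interactable object with an Active state that flips each time it is acted upon.
; Act calls ToggleActive, which inverts Active and then calls Lowlight.
; The Lowlight override runs the parent's version only while inactive, so an active object skips being lowlighted.
; Restart clears Active, lowlights the object and re-enables actor collision.
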(event Custom|Restart
  (Variables|Default|SetActive false)
  (CallFunction|Lowlight)
  (Collision|SetActorEnableCollision true))

(event EventAct
  (CallFunction|ToggleActive))

(event EventLowlight
  (if (not (Variables|Default|GetActive))
    (|CallParentFunction)))

(fn ConstructionScript
  (|CallParentFunction))

(fn ToggleActive
  (Variables|Default|SetActive (not (Variables|Default|GetActive)))
  (CallFunction|Lowlight))