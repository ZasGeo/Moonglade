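; BP_InteractParent is a base Blueprint for interactable objects, with empty Act, Yes and Close events, presumably overridden by children.
; The construction script creates a dynamic material instance from the mesh's first material slot.
; Highlight and Lowlight switch that material's Power parameter between interact and default emissive values.
; End fires CallEndOfAction to signal that the interaction has finished.
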(event Custom|Close)

(event Custom|Yes)

(event Custom|Act)

(fn ConstructionScript
  (bind _mesh (Variables|Default|GetMesh))
  (bind _returnvalue (Rendering|Material|CreateDynamicMaterialInstance _mesh 0 (Rendering|Material|GetMaterial _mesh 0) :!class /Script/Engine.PrimitiveComponent))
  (Variables|Default|SetMaterial _returnvalue))

(fn Highlight
  (Rendering|Material|SetScalarParameterValue (Variables|Default|GetMaterial) "Power" (Variables|Default|GetInteractEmissive) :!class /Script/Engine.MaterialInstanceDynamic))

(fn Lowlight
  (Rendering|Material|SetScalarParameterValue (Variables|Default|GetMaterial) "Power" (Variables|Default|GetDefaultEmissive) :!class /Script/Engine.MaterialInstanceDynamic))

(fn End
  (Default|CallEndOfAction))