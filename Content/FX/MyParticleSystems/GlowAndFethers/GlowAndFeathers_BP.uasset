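; Ambient FX actor that spawns glow rays and falling feathers inside a box volume sized by KillBoxScale.
; On BeginPlay it attaches the feather emitter and starts looping timers for both effects, which act only while recently rendered.
; Beam ticks spawn rays between random points on the box's top and bottom.
; Feather ticks randomize upper-box location and vertical velocity parameters, deriving lifetime from fall distance over speed.
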(event EventBeginPlay
  (CallFunction|BeamandFeathersSetup))

(event EventTick
  (params (DeltaSeconds :type Float%20%28single-precision%29)))

(fn ConstructionScript
  (bind _killboxscale (Variables|Default|GetKillBoxScale))
  (Transformation|SetWorldScale3D (Variables|Default|GetKillBoxCube) _killboxscale)
  (Variables|Default|SetFeathersRange (* _killboxscale 50)))

(fn GetNewBeamSourceandTarget
  (bind _feathersrange (Variables|Default|GetFeathersRange))
  (bind _returnvalue (* _feathersrange "1.000000,1.000000,0.000000"))
  (bind _returnvalue_2 (* _feathersrange "0, 0,1.000000"))
  (bind _returnvalue_3 (* _returnvalue -1))
  (bind _result (Utilities|RandomVectorinRange _returnvalue_3 _returnvalue))
  (return (+ _result _returnvalue_2) (+ _result (* _returnvalue_2 -1))))

(fn SpawnNewBeam
  (if (Class|Actor|WasRecentlyRendered 0.2)
    (bind (_source _target) (CallFunction|GetNewBeamSourceandTarget))
    (bind _returnvalue (Effects|SpawnEmitterAttached "/Game/FX/MyParticleSystems/GlowAndFethers/GlowRay_PS.GlowRay_PS" (Variables|Default|GetKillBoxCube) "None" "0, 0, 0" "0, 0, 0" "SnapToTarget"))
    (Effects|Components|ParticleSystem|SetVectorParameter _returnvalue "Size" (Math|Vector|MakeVector (Variables|Default|GetBeamSize) 0.0 0.0))
    (Effects|Components|ParticleSystem|SetVectorParameter _returnvalue "Source" _source)
    (Effects|Components|ParticleSystem|SetVectorParameter _returnvalue "Target" _target)))

(fn UpdateFeathers
  (bind _feathersps (Variables|Default|GetFeathersPS))
  (bind _feathersrange (Variables|Default|GetFeathersRange))
  (bind _feathersspawnheight (Variables|Default|GetFeathersSpawnHeight))
  (bind _feathersvelocityz (Variables|Default|GetFeathersVelocityZ))
  (bind (_x _y _z) (Math|Vector|BreakVector _feathersrange))
  (bind (_x_2 _y_2) (Math|Vector2D|BreakVector2D _feathersvelocityz))
  (bind _returnvalue (- _z _feathersspawnheight))
  (bind _returnvalue_2 (* -1 _y))
  (bind _returnvalue_3 (* -1 _x))
  (bind _returnvalue_4 (Math|Vector|MakeVector 0.0 0.0 _x_2))
  (bind _returnvalue_5 (Math|Vector|MakeVector 0.0 0.0 _y_2))
  (bind _returnvalue_6 (Math|Vector|MakeVector _returnvalue_3 _returnvalue_2 _returnvalue))
  (bind _result (Utilities|RandomVectorinRange _returnvalue_4 _returnvalue_5))
  (bind _result_2 (Utilities|RandomVectorinRange _returnvalue_6 _feathersrange))
  (if (Class|Actor|WasRecentlyRendered 0.2)
    (Effects|Components|ParticleSystem|SetVectorParameter _feathersps "FeathersLocation" _result_2)
    (Effects|Components|ParticleSystem|SetVectorParameter _feathersps "Velocity" _result)
    (Effects|Components|ParticleSystem|SetFloatParameter _feathersps "Lifetime" (/ (- (.Z (Math|Vector|BreakVector _result_2)) (* -1 (.Z (Math|Vector|BreakVector (Variables|Default|GetFeathersRange))))) (Math|Float|Absolute(Float) (.Z (Math|Vector|BreakVector _result)))))))

(fn BeamandFeathersSetup
  (bind _feathersrange (Variables|Default|GetFeathersRange))
  (bind _feathersspawnrate (Variables|Default|GetFeathersSpawnRate))
  (Utilities|Time|SetTimerbyFunctionName 0 "SpawnNewBeam" (/ 1.0 (Variables|Default|GetBeamSpawnRate)) true)
  (bind _returnvalue (Effects|SpawnEmitterAttached "/Game/FX/MyParticleSystems/GlowAndFethers/Feathers_PS.Feathers_PS" (Variables|Default|GetDefaultSceneRoot) "None"))
  (bind _output_get (Variables|Default|SetFeathersPS _returnvalue))
  (Effects|Components|ParticleSystem|SetFloatParameter _output_get "SpawnRate" _feathersspawnrate)
  (Effects|Components|ParticleSystem|SetVectorParameter _output_get "KillBoxLowerLeft" _feathersrange)
  (Effects|Components|ParticleSystem|SetVectorParameter _output_get "KillBoxUpperRight" (* _feathersrange -1))
  (Effects|Components|ParticleSystem|SetVectorParameter _output_get "SizeScale" (Math|Conversions|ToVector(Vector2D) (Variables|Default|GetFeathersScale)))
  (Utilities|Time|SetTimerbyFunctionName 0 "UpdateFeathers" (/ 1.0 _feathersspawnrate) true))