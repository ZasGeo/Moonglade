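; Child Blueprint of a glow-and-feathers particle effect that runs beam and feather setup on BeginPlay.
; It overrides beam placement, deriving endpoints from the parent's source and FeathersRange, with height and target X offsets driven by source X.
; Beams farther from center in X get shorter, down to a clamped minimum.
; Helper functions trim both segment ends using the section formula for dividing a line in a ratio.
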(event EventBeginPlay
  (CallFunction|BeamandFeathersSetup))

(event EventTick
  (params (DeltaSeconds :type Float%20%28single-precision%29)))

(fn ConstructionScript
  (|CallParentFunction))

(fn GetNewBeamSourceandTarget
  (bind _source (|CallParentFunction))
  (bind (_new_start _new_end) (CallFunction|ShortenSegmentonBothEnds (+ _source (Math|Vector|MakeVector 0.0 0.0 (/ (Math|Float|Absolute(Float) (.X (Math|Vector|BreakVector _source))) 2.0))) (+ (* (Variables|Default|GetFeathersRange) "0.000000, 0,-1.000000") (Math|Vector|MakeVector 0.0 0.0 (/ (Math|Float|Absolute(Float) (.X (Math|Vector|BreakVector _source))) 2.0)) (Math|Vector|MakeVector (/ (.X (Math|Vector|BreakVector _source)) 4.0) 0.0 0.0)) (Math|Float|Clamp(Float) (Class|KismetMathLibrary|InverseLerp (.X (Math|Vector|BreakVector (Variables|Default|GetFeathersRange))) 0.0 (/ (Math|Float|Absolute(Float) (.X (Math|Vector|BreakVector _source))) 2.0)) 0.4 1.0)))
  (return _new_start _new_end))

(fn ShortenSegment
  (params (Start :type Vector) (End :type Vector) (Scale :type Float%20%28single-precision%29))
  (bind (_x _y _z) (Math|Vector|BreakVector Start))
  (bind (_x_2 _y_2 _z_2) (Math|Vector|BreakVector End))
  (return (Math|Vector|MakeVector (Utilities|ShortenSegmentHelper _x _x_2 Scale) (Utilities|ShortenSegmentHelper _y _y_2 Scale) (Utilities|ShortenSegmentHelper _z _z_2 Scale))))

(fn ShortenSegmentonBothEnds
  (params (Start :type Vector) (End :type Vector) (Scale :type Float%20%28single-precision%29))
  (bind _returnvalue (- 1.0 Scale))
  (bind _returnvalue_2 (/ _returnvalue 2.0))
  (bind _returnvalue_3 (- 1.0 _returnvalue_2))
  (bind _returnvalue_4 (/ _returnvalue_3 _returnvalue_2))
  (if (Math|Float|NearlyEqual(Float) Scale 1.0 1e-06)
    (return Start End)
    (elif (Math|Float|NearlyEqual(Float) Scale 0.0 1e-06)
      (return Start Start)
      (else
        (bind _new_end (CallFunction|ShortenSegment Start End _returnvalue_4))
        (bind _new_end_2 (CallFunction|ShortenSegment End Start _returnvalue_4))
        (return _new_end_2 _new_end)))))