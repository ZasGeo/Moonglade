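; BP_Fireflies is a firefly effect actor that scatters particle spawn positions inside a scalable box volume.
; The construction script passes SpawnRate to the particle system, scales the Bounds component and derives half-extents from that scale.
; At BeginPlay, a looping timer running at SpawnRate times per second picks a random offset within those extents and writes it to the particle system's Location parameter.
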(event EventBeginPlay
  (Utilities|Time|SetTimerbyFunctionName 0 "UpdateParticlePosition" (/ 1.0 (Variables|Default|GetSpawnRate)) true))

(fn ConstructionScript
  (bind _bounds_scale (Variables|Default|GetBounds%20Scale))
  (Effects|Components|ParticleSystem|SetFloatParameter (Variables|Emitter|GetParticleSystemComponent) "SpawnRate" (Variables|Default|GetSpawnRate))
  (Transformation|SetWorldScale3D (Variables|Default|GetBounds) _bounds_scale)
  (Variables|Default|Setoffset (* _bounds_scale 5e+01)))

(fn GetNewParticlePosition
  (bind _offset (Variables|Default|Getoffset))
  (bind _returnvalue (* _offset -1))
  (bind (_x _y _z) (Math|Vector|BreakVector _offset))
  (bind (_x_2 _y_2 _z_2) (Math|Vector|BreakVector _returnvalue))
  (return (Math|Vector|MakeVector (Math|Random|RandomFloatinRange _x_2 _x) (Math|Random|RandomFloatinRange _y_2 _y) (Math|Random|RandomFloatinRange _z_2 _z))))

(fn UpdateParticlePosition
  (bind _position (CallFunction|GetNewParticlePosition))
  (Effects|Components|ParticleSystem|SetVectorParameter (Variables|Emitter|GetParticleSystemComponent) "Location" _position))